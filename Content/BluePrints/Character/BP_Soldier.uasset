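; BP_Soldier is the player soldier character, handling health, hazards, weapon pickup, deployables and player HUD widgets.
; Input events destroy enemy spawns by holding, measure range by trace, zoom aim on a timer, and place mortars or cooldown-limited respawn points using BP_Controller's PlayerHand.
; Tick drives camera shake and sphere-trace highlighting of pickups, which spawn and attach Thompson or Garand weapons.
; Overlaps trigger drowning and burning damage; death enables ragdoll and an overhead camera.
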(event OnComponentBeginOverlap(Mesh)
  (params (OverlappedComponent :type Primitive%20Component%20Object%20Reference) (OtherActor :type Actor%20Object%20Reference) (OtherComp :type Primitive%20Component%20Object%20Reference) (OtherBodyIndex :type Integer) (bFromSweep :type Boolean) (SweepResult :type Hit%20Result%20Structure%20%28by%20ref%29)))

(event Custom|CameraShake
  (bind _returnvalue (Game|GetPlayerController 0))
  ;[0.15 0.15 0.15 0.5] 相机抖动
  (if (<= (Math|Vector|VectorLength (Transformation|GetVelocity)) 0.0)
    (Game|Feedback|ClientStartCameraShake _returnvalue "/Game/BluePrints/CameraShake/BP_CameraShake_Idle.BP_CameraShake_Idle_C" 1.0 "CameraLocal" "0, 0, 0")
    (elif (> (Math|Vector|VectorLength (Transformation|GetVelocity)) 6e+02)
      (Game|Feedback|ClientStartCameraShake _returnvalue "/Game/BluePrints/CameraShake/BP_CameraShake_Rush.BP_CameraShake_Rush_C" 1.0 "CameraLocal" "0, 0, 0")
      (else
        (Game|Feedback|ClientStartCameraShake _returnvalue "/Game/BluePrints/CameraShake/BP_CameraShake_Walk.BP_CameraShake_Walk_C" 1.0 "CameraLocal" "0, 0, 0")))))

(event Custom|die
  ;[0.15 0.15 0.15 0.5] 溺水
  (Utilities|Time|ClearandInvalidateTimerbyHandle (stale Collision|EventActorBeginOverlap _returnvalue_2))
  (Widget|RemovefromParent (Variables|Default|Getdrowui))
  (Game|Damage|ApplyDamage self 1e+02 0 0))

(event Custom|PickUpOutline
  ;[0.15 0.15 0.15 0.5] 高亮
  (bind (_outhit _returnvalue) (CallFunction|RangeDetectionOfPicking))
  (if _returnvalue
    (bind _hit_actor (Variables|Default|GetHit%20Actor)
      (:then
        (if (not (== _hit_actor (.HitActor (Collision|BreakHitResult _outhit))))
          (Class|APIDroppen|TurnOffHighlighting(Message) (Variables|Default|GetHit%20Actor))
          (bind _output_get (Variables|Default|SetHit%20Actor (.HitActor (Collision|BreakHitResult _outhit)) :!label _label))
          (Class|APIDroppen|TurnonHighlighting(Message) _output_get)
          (Variables|Default|SetHitActor true)))
      (:else
        (goto _label)))
    (else
      (bind _hit_actor_2 (Variables|Default|GetHit%20Actor)
        (:then
          (Class|APIDroppen|TurnOffHighlighting(Message) _hit_actor_2)
          (Variables|Default|SetHit%20Actor 0)
          (Variables|Default|SetHitActor false))
        (:else)))))

(event Custom|部署冷却
  ;[0.15 0.15 0.15 0.5] 设置重生点
  (bind _result (Math|Integer|DecrementInt (Variables|Default|GetRespawnCold))
    (:%20%20
      (Variables|Default|SetRespawnCold _result))))

(event Custom|部署冷却2
  ;[0.15 0.15 0.15 0.5] 设置重生点
  (bind _result (Math|Integer|DecrementInt (Variables|Default|GetRespawnCold))
    (:%20%20
      (Variables|Default|SetRespawnCold _result))))

(event Custom|EnableRagdoll
  (bind _returnvalue (Utilities|Name|MakeLiteralName "pelvis"))
  (bind _mesh (Variables|Character|GetMesh))
  (Pawn|Components|CharacterMovement|SetMovementMode (Variables|Character|GetCharacterMovement) "MOVE_None" 0)
  (Collision|SetCollisionProfileName _mesh "ragdoll" true :!class /Script/Engine.PrimitiveComponent)
  (Class|SkeletalMeshComponent|SetAllBodiesBelowSimulatePhysics _mesh _returnvalue true true)
  (Class|SkeletalMeshComponent|SetAllBodiesBelowPhysicsBlendWeight (Variables|Character|GetMesh) _returnvalue 1.0 false true))

(event Custom|燃烧
  ;[0.15 0.15 0.15 0.5] 着火灭火
  (Game|Damage|ApplyDamage self 5.0 0 0)
  (Development|PrintString "burn")
  (if (not (>= (Variables|Default|GetHealth) 0.0))
    (Utilities|Time|ClearandInvalidateTimerbyHandle (stale Collision|EventActorEndOverlap _returnvalue_2))
    (Utilities|IsValid (stale Collision|EventActorEndOverlap _returnvalue)
      (:Is%20Valid
        (Components|DestroyComponent (stale Collision|EventActorEndOverlap _returnvalue))))))

(event Custom|火中燃烧
  (if (and (>= (Variables|Default|GetHealth) 0.0) (Variables|Default|Getburn?))
    (CallFunction|燃烧)
    (Utilities|FlowControl|Delay 0.5)
    (else
      (Variables|Default|Setburn? false))))

(event Custom|停止精确瞄准
  ;[0.15 0.15 0.15 0.5] 精确瞄准
  (if (Variables|Default|Get精确瞄准?)
    (Variables|Default|Set精确瞄准? false)
    (bind _新建轨道_0 (Timeline|时间轴_0 PlayFromStart)
      (:Update
        (Camera|SetFieldOfView (Variables|Default|GetCamera) (Math|Float|Lerp 4e+01 (Variables|Default|Get视场) _新建轨道_0))
        (Utilities|Time|ClearandInvalidateTimerbyHandle (stale Input|EnhancedActionEvents|EnhancedInputActionIA_Rush _returnvalue))))))

(event Input|EnhancedActionEvents|EnhancedInputActionIA_SetRespawn
  (params (ActionValue :type Boolean) (ElapsedSeconds :type Float%20%28double-precision%29) (TriggeredSeconds :type Float%20%28double-precision%29) (InputAction :type Input%20Action%20Object%20Reference :default "/Game/Input/IA_SetRespawn.IA_SetRespawn"))
  (bind _setmortarui (Variables|Default|GetSetMortarUI))
  ;[0.15 0.15 0.15 0.5] 设置重生点
  (:Started
    (bind _returnvalue (Actor|GetActorOfClass "/Game/BluePrints/BP_Controller.BP_Controller_C"))
    (Variables|/Game/BluePrints/BP_Controller.BP_Controller_C|SetPlayerHand _returnvalue "NewEnumerator1")
    (UserInterface|Viewport|AddtoViewport (Variables|Default|GetSetRespawnUI) 0)
    (Utilities|IsValid _setmortarui
      (:Is%20Valid
        (Widget|RemovefromParent _setmortarui)
        (bind _returnvalue_2 (Actor|GetActorOfClass "/Game/BluePrints/BP_Controller.BP_Controller_C"))
        (Widget|RemovefromParent (Variables|/Game/BluePrints/BP_Controller.BP_Controller_C|Getbandege _returnvalue_2))
        (Default|使空手 _returnvalue_2)))))

(event Input|EnhancedActionEvents|EnhancedInputActionIA_SetMortar
  (params (ActionValue :type Boolean) (ElapsedSeconds :type Float%20%28double-precision%29) (TriggeredSeconds :type Float%20%28double-precision%29) (InputAction :type Input%20Action%20Object%20Reference :default "/Game/Input/IA_SetMortar.IA_SetMortar"))
  (bind _setrespawnui (Variables|Default|GetSetRespawnUI))
  ;[0.15 0.15 0.15 0.5] 放置迫击炮
  (:Started
    (bind _returnvalue (Actor|GetActorOfClass "/Game/BluePrints/BP_Controller.BP_Controller_C"))
    (Variables|/Game/BluePrints/BP_Controller.BP_Controller_C|SetPlayerHand _returnvalue "NewEnumerator2")
    (UserInterface|Viewport|AddtoViewport (Variables|Default|GetSetMortarUI) 0)
    (Utilities|IsValid _setrespawnui
      (:Is%20Valid
        (Widget|RemovefromParent _setrespawnui)
        (bind _returnvalue_2 (Actor|GetActorOfClass "/Game/BluePrints/BP_Controller.BP_Controller_C"))
        (Widget|RemovefromParent (Variables|/Game/BluePrints/BP_Controller.BP_Controller_C|Getbandege _returnvalue_2))
        (Default|使空手 _returnvalue_2)))))

(event Input|EnhancedActionEvents|EnhancedInputActionIA_PickUp
  (params (ActionValue :type Boolean) (ElapsedSeconds :type Float%20%28double-precision%29) (TriggeredSeconds :type Float%20%28double-precision%29) (InputAction :type Input%20Action%20Object%20Reference :default "/Game/Input/IA_PickUp.IA_PickUp"))
  ;[0.15 0.15 0.15 0.5] 捡枪
  (:Started
    (Variables|Default|GetHit%20Actor
      (:then
        (bind _asset (Class|APIDroppen|GetWeaponDataAsset(Message) (Variables|Default|GetHit%20Actor)))
        (bind _returnvalue (Game|SpawnActorfromClass (Variables|/Game/BluePrints/weapon/BP_Weapon.BP_Weapon_C|GetWeaponClass _asset) (Math|Transform|MakeTransform "0, 0, 0" "0, 0, 0" "1.000000,1.000000,1.000000") "Undefined" "MultiplyWithRoot" 0 _asset 0))
        (switch Utilities|FlowControl|Switch|SwitchonENUM_WeaponType (.weapontype (Variables|/Game/BluePrints/weapon/BP_Weapon.BP_Weapon_C|GetWeaponAttri _asset))
          (:NewEnumerator0
            (bind _output_get (Variables|Default|SetEquippedThompson _returnvalue))
            (bind _returnvalue_2 (Utilities|Attach _output_get))
            (if _returnvalue_2
              (Actor|DestroyActor (Variables|Default|GetHit%20Actor))
              (Variables|Default|SetHit%20Actor 0)
              (for _array_element (Variables|Default|GetbackWeapons)
                (Actor|DestroyActor _array_element))
              (Variables|Default|SetbackWeapons (Actor|GetAttachedActors true false))
              (bind _asbp_controller (Utilities|Casting|CastToBP_Controller (Game|GetPlayerController 0)))
              (Variables|/Game/BluePrints/BP_Controller.BP_Controller_C|SetThompsonAllBullet _asbp_controller 150)))
          (:NewEnumerator1
            (bind _output_get_2 (Variables|Default|SetEquippedGarand _returnvalue))
            (bind _returnvalue_3 (Utilities|Attach _output_get_2))
            (if _returnvalue_3
              (Actor|DestroyActor (Variables|Default|GetHit%20Actor))
              (Variables|Default|SetHit%20Actor 0)
              (for _array_element_2 (Variables|Default|GetbackWeaponsG)
                (Actor|DestroyActor _array_element_2))
              (Variables|Default|SetbackWeaponsG (Actor|GetAttachedActors true false))
              (bind _asbp_controller_2 (Utilities|Casting|CastToBP_Controller (Game|GetPlayerController 0)))
              (Variables|/Game/BluePrints/BP_Controller.BP_Controller_C|SetGarandAllBullet _asbp_controller_2 48)))))
      (:else))))

(event Input|EnhancedActionEvents|EnhancedInputActionIA_distance
  (params (ActionValue :type Boolean) (ElapsedSeconds :type Float%20%28double-precision%29) (TriggeredSeconds :type Float%20%28double-precision%29) (InputAction :type Input%20Action%20Object%20Reference :default "/Game/Input/IA_distance.IA_distance"))
  (bind _returnvalue (Game|GetPlayerCameraManager 0))
  (bind _arrow2 (Variables|Default|GetArrow2))
  (bind _returnvalue_2 (Transformation|GetActorLocation _returnvalue))
  (bind _returnvalue_3 (Transformation|GetWorldLocation _arrow2))
  ;[0.15 0.15 0.15 0.5] 测距
  (:Started
    (Utilities|FlowControl|DoOnce false :!label _label
      (:Completed
        (bind (_outhit _returnvalue_4) (Collision|LineTraceByChannel _returnvalue_2 (+ _returnvalue_2 (* (Transformation|GetActorForwardVector _returnvalue) "99999.000000,99999.000000,99999.000000")) "TraceTypeQuery6" false 0 "None"))
        (if _returnvalue_4
          (Variables|Default|SetOut%20Hit%20Location (.location _outhit))
          (Variables|Default|Setdistance (Math|Float|Round (/ (Math|Float|Sqrt (+ (Math|Float|Square (- (.x (Variables|Default|GetOut%20Hit%20Location)) (.x _returnvalue_3))) (Math|Float|Square (- (.y (Variables|Default|GetOut%20Hit%20Location)) (.y _returnvalue_3))) (Math|Float|Square (- (.z (Variables|Default|GetOut%20Hit%20Location)) (.z _returnvalue_3))))) 1e+02)))
          (bind _returnvalue_5 (UserInterface|CreateWidget "/Game/UI/WBP_distance.WBP_distance_C"))
          (UserInterface|Viewport|AddtoViewport _returnvalue_5 0)
          (Utilities|FlowControl|Delay 1.0)
          (Widget|RemovefromParent _returnvalue_5)
          (goto _label Reset)
          (else
            (goto _label Reset)))))))

(event Input|EnhancedActionEvents|EnhancedInputActionIA_PickUp
  (params (ActionValue :type Boolean) (ElapsedSeconds :type Float%20%28double-precision%29) (TriggeredSeconds :type Float%20%28double-precision%29) (InputAction :type Input%20Action%20Object%20Reference :default "/Game/Input/IA_PickUp.IA_PickUp"))
  (bind _scene (Variables|Default|GetScene))
  (bind _coldui (Variables|Default|Getcoldui))
  (bind _returnvalue (Transformation|GetWorldTransform _scene))
  ;[0.15 0.15 0.15 0.5] 设置重生点
  (:Started
    (bind _returnvalue_2 (Actor|GetActorOfClass "/Game/BluePrints/BP_Controller.BP_Controller_C"))
    (switch Utilities|FlowControl|Switch|Switchonplayerhand (Variables|/Game/BluePrints/BP_Controller.BP_Controller_C|GetPlayerHand _returnvalue_2)
      (:NewEnumerator1
        (bind _outactors (Actor|GetAllActorsOfClass "/Game/BluePrints/testbp/spawn.spawn_C"))
        (if (> (Utilities|Array|Length _outactors) 0)
          (if (< (Variables|Default|GetRespawnCold) 1)
            (Variables|Default|SetRespawnCold 20)
            (bind _returnvalue_3 (Actor|GetActorOfClass "/Game/BluePrints/testbp/spawn.spawn_C"))
            (Actor|DestroyActor _returnvalue_3)
            (Game|SpawnActorfromClass "/Game/BluePrints/testbp/spawn.spawn_C" _returnvalue "Undefined" "MultiplyWithRoot" 0 0)
            (bind _returnvalue_4 (Utilities|Time|SetTimerbyEvent (delegate Custom|部署冷却) 1.0 true))
            (Utilities|FlowControl|Delay 2e+01)
            (Utilities|Time|ClearandInvalidateTimerbyHandle _returnvalue_4)
            (Variables|Default|SetRespawnCold 0)
            (else
              (Default|冷却 (Variables|Default|Getcoldui))
              (UserInterface|Viewport|AddtoViewport _coldui 0)
              (Utilities|FlowControl|Delay 0.5)
              (Widget|RemovefromParent _coldui)))
          (else
            (Variables|Default|SetRespawnCold 20)
            (Game|SpawnActorfromClass "/Game/BluePrints/testbp/spawn.spawn_C" _returnvalue "Undefined" "MultiplyWithRoot" 0 0)
            (bind _returnvalue_5 (Utilities|Time|SetTimerbyEvent (delegate Custom|部署冷却2) 1.0 true))
            (Utilities|FlowControl|Delay 2e+01)
            (Utilities|Time|ClearandInvalidateTimerbyHandle _returnvalue_5)
            (Variables|Default|SetRespawnCold 0)))))))

(event Input|EnhancedActionEvents|EnhancedInputActionIA_PickUp
  (params (ActionValue :type Boolean) (ElapsedSeconds :type Float%20%28double-precision%29) (TriggeredSeconds :type Float%20%28double-precision%29) (InputAction :type Input%20Action%20Object%20Reference :default "/Game/Input/IA_PickUp.IA_PickUp"))
  (bind _cantsetui (Variables|Default|GetCantSetUI))
  ;[0.15 0.15 0.15 0.5] 放置迫击炮
  (:Started
    (bind _returnvalue (Actor|GetActorOfClass "/Game/BluePrints/BP_Controller.BP_Controller_C"))
    (switch Utilities|FlowControl|Switch|Switchonplayerhand (Variables|/Game/BluePrints/BP_Controller.BP_Controller_C|GetPlayerHand _returnvalue)
      (:NewEnumerator2
        (bind _outactors (Actor|GetAllActorsOfClass "/Game/BluePrints/mortar.mortar_C"))
        (bind _returnvalue_2 (Game|SpawnActorfromClass "/Game/BluePrints/mortar.mortar_C" (Transformation|GetWorldTransform (Variables|Default|GetArrow1)) "Undefined" "MultiplyWithRoot" 0 0))
        (Utilities|IsValid _returnvalue_2
          (:Is%20Valid
            (if (not (== (Utilities|Array|Length _outactors) 0))
              (Actor|DestroyActor _outactors)))
          (:Is%20Not%20Valid
            (UserInterface|Viewport|AddtoViewport _cantsetui 0)
            (Utilities|FlowControl|Delay 0.5)
            (Widget|RemovefromParent _cantsetui)))))))

(event Input|EnhancedActionEvents|EnhancedInputActionIA_Rush
  (params (ActionValue :type Boolean) (ElapsedSeconds :type Float%20%28double-precision%29) (TriggeredSeconds :type Float%20%28double-precision%29) (InputAction :type Input%20Action%20Object%20Reference :default "/Game/Input/IA_Rush.IA_Rush"))
  (bind _camera (Variables|Default|GetCamera))
  ;[0.15 0.15 0.15 0.5] 精确瞄准
  (:Started
    (if (Variables|Default|GetIsAiming)
      (Utilities|Time|ClearandInvalidateTimerbyHandle (stale _returnvalue))
      (Variables|Default|Set视场 (Variables|/Script/Engine.CameraComponent|GetFieldOfView _camera))
      (Variables|Default|Set精确瞄准? true)
      (bind _新建轨道_0 (Timeline|精确瞄准 PlayFromStart)
        (:Update
          (Camera|SetFieldOfView _camera (Math|Float|Lerp (Variables|Default|Get视场) 4e+01 _新建轨道_0))
          (bind _returnvalue (Utilities|Time|SetTimerbyEvent (delegate Custom|停止精确瞄准) 5.0))))))
  (:Canceled
    (if (Variables|Default|GetIsAiming) :!label _label
      (if (Variables|Default|Get精确瞄准?)
        (Utilities|Time|ClearandInvalidateTimerbyHandle _returnvalue)
        (Variables|Default|Set精确瞄准? false)
        (bind _新建轨道_0_2 (Timeline|时间轴 PlayFromStart)
          (:Update
            (Camera|SetFieldOfView _camera (Math|Float|Lerp 4e+01 (Variables|Default|Get视场) _新建轨道_0_2)))))))
  (:Completed
    (goto _label)))

(event Input|EnhancedActionEvents|EnhancedInputActionIA_1
  (params (ActionValue :type Boolean) (ElapsedSeconds :type Float%20%28double-precision%29) (TriggeredSeconds :type Float%20%28double-precision%29) (InputAction :type Input%20Action%20Object%20Reference :default "/Game/Input/IA_1.IA_1"))
  (:Started
    (Widget|RemovefromParent (Variables|Default|GetSetRespawnUI))
    (Widget|RemovefromParent (Variables|Default|GetSetMortarUI))
    (bind _returnvalue (Actor|GetActorOfClass "/Game/BluePrints/BP_Controller.BP_Controller_C"))
    (Widget|RemovefromParent (Variables|/Game/BluePrints/BP_Controller.BP_Controller_C|Getbandege _returnvalue))))

(event Input|EnhancedActionEvents|EnhancedInputActionIA_2
  (params (ActionValue :type Boolean) (ElapsedSeconds :type Float%20%28double-precision%29) (TriggeredSeconds :type Float%20%28double-precision%29) (InputAction :type Input%20Action%20Object%20Reference :default "/Game/Input/IA_2.IA_2"))
  (:Started
    (Widget|RemovefromParent (Variables|Default|GetSetRespawnUI))
    (Widget|RemovefromParent (Variables|Default|GetSetMortarUI))
    (bind _returnvalue (Actor|GetActorOfClass "/Game/BluePrints/BP_Controller.BP_Controller_C"))
    (Widget|RemovefromParent (Variables|/Game/BluePrints/BP_Controller.BP_Controller_C|Getbandege _returnvalue))))

(event Input|EnhancedActionEvents|EnhancedInputActionIA_3
  (params (ActionValue :type Boolean) (ElapsedSeconds :type Float%20%28double-precision%29) (TriggeredSeconds :type Float%20%28double-precision%29) (InputAction :type Input%20Action%20Object%20Reference :default "/Game/Input/IA_3.IA_3"))
  (:Started
    (Widget|RemovefromParent (Variables|Default|GetSetRespawnUI))
    (Widget|RemovefromParent (Variables|Default|GetSetMortarUI))
    (bind _returnvalue (Actor|GetActorOfClass "/Game/BluePrints/BP_Controller.BP_Controller_C"))
    (Widget|RemovefromParent (Variables|/Game/BluePrints/BP_Controller.BP_Controller_C|Getbandege _returnvalue))))

(event Input|EnhancedActionEvents|EnhancedInputActionIA_PickUp
  (params (ActionValue :type Boolean) (ElapsedSeconds :type Float%20%28double-precision%29) (TriggeredSeconds :type Float%20%28double-precision%29) (InputAction :type Input%20Action%20Object%20Reference :default "/Game/Input/IA_PickUp.IA_PickUp"))
  (bind _destoryenemyspawnui (Variables|Default|GetDestoryEnemySpawnUI))
  ;[0.15 0.15 0.15 0.5] 摧毁敌方出生点
  (:Triggered
    (bind _returnvalue (Actor|GetActorOfClass "BP_Soldier_C"))
    (for _array_element (Collision|GetOverlappingActors _returnvalue "/Game/BluePrints/testbp/EnemySpawn.EnemySpawn_C" :!class /Script/Engine.Actor)
      (Utilities|IsValid _array_element
        (:Is%20Valid
          (UserInterface|Viewport|AddtoViewport _destoryenemyspawnui 0)
          (if (>= (Variables|Default|GetDestoryBar) 1.0)
            (Actor|DestroyActor _array_element)
            (Widget|RemovefromParent _destoryenemyspawnui)
            (Widget|RemovefromParent (Variables|Default|GetDestoryIntroductionUI))
            (else
              (Utilities|FlowControl|DoOnce false :!label _label
                (:Completed
                  (Variables|Default|SetDestoryBar (+ (Variables|Default|GetDestoryBar) 0.04))
                  (Utilities|FlowControl|Delay 0.2)
                  (goto _label Reset)))))))))
  (:Completed
    (Variables|Default|SetDestoryBar 0.0)
    (Utilities|IsValid _destoryenemyspawnui
      (:Is%20Valid
        (Widget|RemovefromParent _destoryenemyspawnui)))))

(event EventBeginPlay
  (bind _returnvalue (UserInterface|CreateWidget "/Game/UI/colddown.colddown_C"))
  (Variables|Default|Setcoldui _returnvalue)
  (bind _returnvalue_2 (UserInterface|CreateWidget "/Game/UI/WBP_AimPoint.WBP_AimPoint_C"))
  (bind _output_get (Variables|Default|SetAim _returnvalue_2))
  (UserInterface|Viewport|AddtoViewport _output_get 0)
  (bind _returnvalue_3 (UserInterface|CreateWidget "/Game/UI/WBP_CantSet.WBP_CantSet_C"))
  (Variables|Default|SetCantSetUI _returnvalue_3)
  (bind _returnvalue_4 (UserInterface|CreateWidget "/Game/UI/WBP_DestoryEnemySpawn.WBP_DestoryEnemySpawn_C"))
  (Variables|Default|SetDestoryEnemySpawnUI _returnvalue_4)
  (bind _returnvalue_5 (UserInterface|CreateWidget "/Game/UI/WBP_PlayerHealth.WBP_PlayerHealth_C"))
  (bind _output_get_2 (Variables|Default|SetPlayerHealthUI _returnvalue_5))
  (UserInterface|Viewport|AddtoViewport _output_get_2 0)
  (bind _returnvalue_6 (UserInterface|CreateWidget "/Game/UI/WBP_SetRespawn.WBP_SetRespawn_C"))
  (Variables|Default|SetSetRespawnUI _returnvalue_6)
  (bind _returnvalue_7 (UserInterface|CreateWidget "/Game/UI/WBP_SetMortar.WBP_SetMortar_C"))
  (Variables|Default|SetSetMortarUI _returnvalue_7)
  (bind _returnvalue_8 (UserInterface|CreateWidget "/Game/UI/WBP_DestoryEnemyIntroduction.WBP_DestoryEnemyIntroduction_C"))
  (Variables|Default|SetDestoryIntroductionUI _returnvalue_8)
  (bind _returnvalue_9 (UserInterface|CreateWidget "/Game/UI/WBP_hurt.WBP_hurt_C"))
  (Variables|Default|SetHurtUI _returnvalue_9)
  (Variables|Default|Setburn? false)
  (Utilities|FlowControl|Sequence
    (:then_0
      (Utilities|FlowControl|Delay 0.2)
      (bind _returnvalue_10 (Actor|GetActorOfClass "/Game/BluePrints/weapon/BP_Camera.BP_Camera_C"))
      (Variables|Default|SetCamera (Variables|/Game/BluePrints/weapon/BP_Camera.BP_Camera_C|GetCamera _returnvalue_10)))))

(event EventTick
  (params (DeltaSeconds :type Float%20%28single-precision%29))
  (Utilities|FlowControl|Sequence
    (:then_0
      (if (Variables|Default|Getshack?)
        (CallFunction|CameraShake)))
    (:then_1
      (CallFunction|PickUpOutline))))

(event Game|Damage|EventAnyDamage
  (params (Damage :type Float%20%28single-precision%29) (DamageType :type Damage%20Type%20Object%20Reference) (InstigatedBy :type Controller%20Object%20Reference) (DamageCauser :type Actor%20Object%20Reference))
  (bind _returnvalue (Game|GetPlayerController 0))
  (bind _returnvalue_2 (Transformation|GetActorTransform))
  (bind _hurtui (Variables|Default|GetHurtUI))
  (Utilities|FlowControl|Sequence
    (:then_0
      (bind _output_get (Variables|Default|SetHealth (- (Variables|Default|GetHealth) Damage)))
      (Class|APIUI|HealthUpdate(Message) (Variables|Default|GetPlayerHealthUI) _output_get (Variables|Default|GetMaxHealth))
      (if (<= (Variables|Default|GetHealth) 0.0)
        (bind _asbp_controller (Utilities|Casting|CastToBP_Controller (Game|GetPlayerController 0)))
        (CallFunction|EnableRagdoll)
        (bind _returnvalue_3 (Game|SpawnActorfromClass "/Game/BluePrints/weapon/BP_Camera.BP_Camera_C" (Math|Transform|MakeTransform (Math|Vector|MakeVector (.x (.location _returnvalue_2)) (.y (.location _returnvalue_2)) (+ (.z (.location _returnvalue_2)) 1e+03)) (Math|Rotator|MakeRotator (.roll (.rotation _returnvalue_2)) (- (.pitch (.rotation _returnvalue_2)) 9e+01) (.yaw (.rotation _returnvalue_2))) "1.000000,1.000000,1.000000") "Undefined" "MultiplyWithRoot" 0 0))
        (Game|Player|SetViewTargetwithBlend _asbp_controller _returnvalue_3 0.0 "VTBlend_EaseInOut" 2.0 false)
        (Utilities|FlowControl|Delay 5.0)
        (UserInterface|Viewport|AddtoViewport (Variables|/Game/BluePrints/BP_Controller.BP_Controller_C|Getdieui _asbp_controller) 0)
        (Input|SetInputModeGameandUI _returnvalue 0 "DoNotLock" true false)
        (Variables|/Script/Engine.PlayerController|SetbShowMouseCursor _returnvalue true)
        (Actor|DestroyActor _returnvalue_3)
        (Game|Player|SetViewTargetwithBlend _asbp_controller self 0.0 "VTBlend_Cubic" 1.0 false)
        (Class|APIUI|HealthUpdate(Message) (Variables|Default|GetPlayerHealthUI) 1e+02 (Variables|Default|GetMaxHealth))))
    (:then_1
      (UserInterface|Viewport|AddtoViewport _hurtui 0)
      (Utilities|FlowControl|Delay 1.0)
      (Default|渐隐动画 _hurtui)
      (Utilities|FlowControl|Delay 0.75)
      (Widget|RemovefromParent _hurtui))))

(event EventSetAITeam
  (params (Team :type ENUM_Team%20Enum :default "NewEnumerator0"))
  (Variables|Default|SetTeam Team))

(event Collision|EventActorBeginOverlap
  (params (OtherActor :type Actor%20Object%20Reference))
  (Utilities|FlowControl|Sequence
    (:then_0
      ;[0.15 0.15 0.15 0.5] 溺水
      (Utilities|Casting|CastTodieheigt OtherActor)
      (bind _returnvalue (UserInterface|CreateWidget "/Game/UI/drow.drow_C"))
      (Variables|Default|Setdrowui _returnvalue)
      (UserInterface|Viewport|AddtoViewport (Variables|Default|Getdrowui) 0)
      (bind _returnvalue_2 (Utilities|Time|SetTimerbyEvent (delegate Custom|die) 3.0)))
    (:then_1
      (if (Actor|ActorHasTag OtherActor "location")
        (Default|CallEnter)))
    (:then_2
      (Variables|Default|Setburn? true)
      (Utilities|Casting|CastTofire OtherActor)
      (bind _returnvalue_3 (Utilities|Time|SetTimerbyEvent (delegate Custom|火中燃烧) 0.5 true)))
    (:then_3
      ;[0.15 0.15 0.15 0.5] 着火灭火
      (Utilities|Casting|CastToWaterBodyOcean OtherActor)
      (Utilities|Time|ClearandInvalidateTimerbyHandle (stale Collision|EventActorEndOverlap _returnvalue_2) :!label _label)
      (Utilities|IsValid (stale Collision|EventActorEndOverlap _returnvalue)
        (:Is%20Valid
          (Components|DestroyComponent (stale Collision|EventActorEndOverlap _returnvalue))
          (Development|PrintString "water"))))
    (:then_4
      (Utilities|Casting|CastToWaterBodyCustom OtherActor)
      (goto _label))))

(event Collision|EventActorEndOverlap
  (params (OtherActor :type Actor%20Object%20Reference))
  (Utilities|FlowControl|Sequence
    (:then_0
      ;[0.15 0.15 0.15 0.5] 溺水
      (Utilities|Casting|CastTodieheigt OtherActor)
      (Utilities|Time|ClearandInvalidateTimerbyHandle (stale Collision|EventActorBeginOverlap _returnvalue_2))
      (Widget|RemovefromParent (Variables|Default|Getdrowui)))
    (:then_1
      (Utilities|FlowControl|Sequence
        (:then_0
          (if (Variables|Default|Getburn?)
            ;[0.15 0.15 0.15 0.5] 着火灭火
            (Utilities|Casting|CastTofire OtherActor)
            (bind _returnvalue (Niagara|SpawnSystemAttached "/Game/BluePrints/effect/FXS_fire1.FXS_fire1" (Variables|Default|GetArrow3) "None" "0, 0, 0" "0, 0, 0" "KeepRelativeOffset" false))
            (bind _returnvalue_2 (Utilities|Time|SetTimerbyEvent (delegate Custom|燃烧) 0.5 true))
            (Utilities|FlowControl|Delay 5.1)
            (Utilities|Time|ClearandInvalidateTimerbyHandle _returnvalue_2)
            (Utilities|IsValid _returnvalue
              (:Is%20Valid
                (Components|DestroyComponent _returnvalue)))))
        (:then_1
          (Utilities|Time|ClearandInvalidateTimerbyHandle (stale Collision|EventActorBeginOverlap _returnvalue_3)))))))

(event Input|KeyboardEvents|9
  (params (Key :type Key%20Structure :default "None"))
  ;[0.15 0.15 0.15 0.5] 死亡测试
  (:Pressed
    (Game|Damage|ApplyDamage self 1e+02 0 0)))

(fn ConstructionScript)

(fn RangeDetectionOfPicking
  (bind _returnvalue (Game|GetPlayerCameraManager 0))
  (bind _returnvalue_2 (Transformation|GetActorLocation _returnvalue))
  (bind (_outhit _returnvalue_3) (Collision|SphereTraceByChannel _returnvalue_2 (+ _returnvalue_2 (* (Transformation|GetActorForwardVector _returnvalue) "350.000000,350.000000,350.000000")) 1e+01 "TraceTypeQuery3" false 0 "None"))
  (return _outhit _returnvalue_3))

(fn GetAITeam
  (return "NewEnumerator0"))

(fn GetEquippedWeaponDataAsset
  (return 0))

(fn GetWeaponDataAsset
  (return 0))