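; Mortar explosion actor that applies area damage to both friendly and enemy AI and plays a Niagara effect.
; 启用 briefly switches on three collision boxes, then 造成伤害 damages their overlapping actors at a separate tier per box, so overlaps stack.
; After delays it disables collision, hides the effect and clears Used, which suggests reuse.
; Box1 is enabled as PhysicsOnly, unlike the other two query-enabled boxes.
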(event Custom|造成伤害
  (bind _box (Variables|Default|GetBox))
  (bind _box1 (Variables|Default|GetBox1))
  (bind _box2 (Variables|Default|GetBox2))
  (Utilities|FlowControl|Sequence
    (:then_0
      (Utilities|FlowControl|Sequence
        (:then_0
          (for _array_element (Collision|GetOverlappingActors _box "/Game/AI/AIBluePrints/BP_FriendAI.BP_FriendAI_C" :!class /Script/Engine.PrimitiveComponent)
            (Game|Damage|ApplyDamage _array_element 65.0 0 0)))
        (:then_1
          (for _array_element_2 (Collision|GetOverlappingActors _box "/Game/AI/AIBluePrints/BP_EAI.BP_EAI_C" :!class /Script/Engine.PrimitiveComponent)
            (Game|Damage|ApplyDamage _array_element_2 65.0 0 0)))))
    (:then_1
      (Utilities|FlowControl|Sequence
        (:then_0
          (for _array_element_3 (Collision|GetOverlappingActors _box1 "/Game/AI/AIBluePrints/BP_FriendAI.BP_FriendAI_C" :!class /Script/Engine.PrimitiveComponent)
            (Game|Damage|ApplyDamage _array_element_3 25.0 0 0)))
        (:then_1
          (for _array_element_4 (Collision|GetOverlappingActors _box1 "/Game/AI/AIBluePrints/BP_EAI.BP_EAI_C" :!class /Script/Engine.PrimitiveComponent)
            (Game|Damage|ApplyDamage _array_element_4 25.0 0 0)))))
    (:then_2
      (Utilities|FlowControl|Sequence
        (:then_0
          (for _array_element_5 (Collision|GetOverlappingActors _box2 "/Game/AI/AIBluePrints/BP_FriendAI.BP_FriendAI_C" :!class /Script/Engine.PrimitiveComponent)
            (Game|Damage|ApplyDamage _array_element_5 1e+01 0 0)
            (Development|PrintString "击中")))
        (:then_1
          (for _array_element_6 (Collision|GetOverlappingActors _box2 "/Game/AI/AIBluePrints/BP_EAI.BP_EAI_C" :!class /Script/Engine.PrimitiveComponent)
            (Game|Damage|ApplyDamage _array_element_6 1e+01 0 0)
            (Development|PrintString "击中")))))))

(event Custom|启用
  (bind _niagara (Variables|Default|GetNiagara))
  (bind _niagara_2 (Variables|Default|GetNiagara))
  (Collision|SetCollisionEnabled (Variables|Default|GetBox) "QueryAndPhysics")
  (Collision|SetCollisionEnabled (Variables|Default|GetBox1) "PhysicsOnly")
  (Collision|SetCollisionEnabled (Variables|Default|GetBox2) "QueryAndPhysics")
  (Transformation|AttachComponentToComponent _niagara_2 (Variables|Default|GetDefaultSceneRoot) "None" "SnapToTarget" "SnapToTarget" "SnapToTarget" true)
  (Components|Activation|Activate _niagara_2 false)
  (Rendering|SetVisibility _niagara_2 true false)
  (CallFunction|造成伤害)
  (Utilities|FlowControl|Delay 0.2)
  (Collision|SetCollisionEnabled (Variables|Default|GetBox) "NoCollision")
  (Collision|SetCollisionEnabled (Variables|Default|GetBox1) "NoCollision")
  (Collision|SetCollisionEnabled (Variables|Default|GetBox2) "NoCollision")
  (Utilities|FlowControl|Delay 4.5)
  (Components|Activation|Deactivate _niagara)
  (Rendering|SetVisibility _niagara false false)
  (Variables|Default|Setused? false))

(event Custom|禁用
  (Collision|SetCollisionEnabled (Variables|Default|GetBox) "NoCollision")
  (Collision|SetCollisionEnabled (Variables|Default|GetBox1) "NoCollision")
  (Collision|SetCollisionEnabled (Variables|Default|GetBox2) "NoCollision")
  (Rendering|SetVisibility (Variables|Default|GetNiagara) true false)
  (Variables|Default|Setused? false))

(event EventTick
  (params (DeltaSeconds :type Float%20%28single-precision%29)))

(event EventBeginPlay
  (CallFunction|禁用))

(fn ConstructionScript)