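; Location zone actor that counts the BP_ai and BP_FriendAI actors overlapping it and responds to BP_Soldier presence.
; Tick refreshes both counts, adds the controller's TotalUI to the viewport once when a soldier overlaps, and rotates its Widget to match the soldier's WidgetArrow.
; Box overlap events switch TotalUI's PlayerState, with end overlap conditionally removing the UI and resetting the DoOnce.
; BeginPlay caches TotalUI from BP_Controller after a short delay.
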(event OnComponentEndOverlap(Box)
  (params (OverlappedComponent :type Primitive%20Component%20Object%20Reference) (OtherActor :type Actor%20Object%20Reference) (OtherComp :type Primitive%20Component%20Object%20Reference) (OtherBodyIndex :type Integer))
  (if (== (Utilities|Array|Length (Collision|GetOverlappingActors OtherActor "/Game/BluePrints/Character/BP_Soldier.BP_Soldier_C" :!class /Script/Engine.Actor)) 0)
    (Variables|/Game/UI/WBP_total.WBP_total_C|SetPlayerState (Variables|Default|GetTotal%20UI) "NewEnumerator0")
    (Widget|RemovefromParent (Variables|Default|GetTotal%20UI))
    (Utilities|FlowControl|DoOnce false) ; enters at Reset
  ))

(event OnComponentBeginOverlap(Box)
  (params (OverlappedComponent :type Primitive%20Component%20Object%20Reference) (OtherActor :type Actor%20Object%20Reference) (OtherComp :type Primitive%20Component%20Object%20Reference) (OtherBodyIndex :type Integer) (bFromSweep :type Boolean) (SweepResult :type Hit%20Result%20Structure%20%28by%20ref%29))
  (Utilities|Casting|CastToBP_Soldier OtherActor)
  (Development|PrintString "Hello")
  (Variables|/Game/UI/WBP_total.WBP_total_C|SetPlayerState (Variables|Default|GetTotal%20UI) "NewEnumerator1"))

(event EventBeginPlay
  (Utilities|FlowControl|Delay 0.2)
  (bind _returnvalue (Actor|GetActorOfClass "/Game/BluePrints/BP_Controller.BP_Controller_C"))
  (Variables|Default|SetTotal%20UI (Variables|/Game/BluePrints/BP_Controller.BP_Controller_C|GetTotalUI _returnvalue)))

(event EventTick
  (params (DeltaSeconds :type Float%20%28single-precision%29))
  (Utilities|FlowControl|Sequence
    (:then_0
      (Variables|Default|SetEnemyNum (Utilities|Array|Length (Collision|GetOverlappingActors "/Game/BluePrints/Character/BP_ai.BP_ai_C" :!class /Script/Engine.Actor))))
    (:then_1
      (if (> (Utilities|Array|Length (Collision|GetOverlappingActors "/Game/BluePrints/Character/BP_Soldier.BP_Soldier_C" :!class /Script/Engine.Actor)) 0)
        (Utilities|FlowControl|DoOnce false
          (:Completed
            (UserInterface|Viewport|AddtoViewport (Variables|Default|GetTotal%20UI) 0)))))
    (:then_2
      (Variables|Default|SetFriendNum (Utilities|Array|Length (Collision|GetOverlappingActors "/Game/BluePrints/Character/BP_FriendAI.BP_FriendAI_C" :!class /Script/Engine.Actor))))
    (:then_3
      (bind _returnvalue (Actor|GetActorOfClass "/Game/BluePrints/Character/BP_Soldier.BP_Soldier_C"))
      (Transformation|SetWorldRotation (Variables|Default|GetWidget) (Transformation|GetWorldRotation (Variables|/Game/BluePrints/Character/BP_Soldier.BP_Soldier_C|GetWidgetArrow _returnvalue)) false false))))

(fn ConstructionScript)