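; location3 is a location zone actor that tracks AI enemies inside it and briefly shows a UI when soldiers are present.
; Shortly after BeginPlay it caches TotalUI from BP_Controller.
; Tick stores the overlapping BP_ai count in EnemyNum and, gated by a DoOnce, shows TotalUI for three seconds when a BP_Soldier overlaps.
; Box end-overlap resets the gate if the departing actor overlaps no soldiers.
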(event OnComponentEndOverlap(Box)
  (params (OverlappedComponent :type Primitive%20Component%20Object%20Reference) (OtherActor :type Actor%20Object%20Reference) (OtherComp :type Primitive%20Component%20Object%20Reference) (OtherBodyIndex :type Integer))
  (bind _total_ui (Variables|Default|GetTotal%20UI))
  (if (== (Utilities|Array|Length (Collision|GetOverlappingActors OtherActor "/Game/BluePrints/Character/BP_Soldier.BP_Soldier_C" :!class /Script/Engine.Actor)) 0)
    (Development|PrintString "111")
    (Utilities|FlowControl|DoOnce false) ; enters at Reset
  ))

(event EventBeginPlay
  (Utilities|FlowControl|Delay 0.2)
  (bind _returnvalue (Actor|GetActorOfClass "/Game/BluePrints/BP_Controller.BP_Controller_C"))
  (Variables|Default|SetTotal%20UI (Variables|/Game/BluePrints/BP_Controller.BP_Controller_C|GetTotalUI _returnvalue)))

(event EventTick
  (params (DeltaSeconds :type Float%20%28single-precision%29))
  (bind _total_ui (Variables|Default|GetTotal%20UI))
  (Utilities|FlowControl|Sequence
    (:then_0
      (Variables|Default|SetEnemyNum (Utilities|Array|Length (Collision|GetOverlappingActors "/Game/BluePrints/Character/BP_ai.BP_ai_C" :!class /Script/Engine.Actor))))
    (:then_1
      (if (> (Utilities|Array|Length (Collision|GetOverlappingActors "/Game/BluePrints/Character/BP_Soldier.BP_Soldier_C" :!class /Script/Engine.Actor)) 0)
        (Utilities|FlowControl|DoOnce false
          (:Completed
            (UserInterface|Viewport|AddtoViewport _total_ui 0)
            (Utilities|FlowControl|Delay 3.0)
            (Utilities|IsValid _total_ui
              (:Is%20Valid
                (Widget|RemovefromParent _total_ui)))))))))

(fn ConstructionScript)