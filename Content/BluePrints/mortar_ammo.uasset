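; Mortar shell projectile that launches its physics Sphere on spawn and spawns a Hit_effect actor where it strikes.
; BeginPlay applies an impulse along the sphere's rotation, scaled by its mass and the initial speed (初速).
; Impacts come from both the Hit event and a per-tick Visibility trace from the previous position, which leaves persistent debug lines.
; Both paths print debug text and share the spawn step, without destroying the shell.
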(event EventBeginPlay
  (bind _sphere (Variables|Default|GetSphere))
  (Physics|AddImpulse _sphere (Math|Vector|RotateVector (Math|Vector|MakeVector (* (* (Physics|GetMass _sphere) (Variables|Default|Get初速)) 5e+01) 0.0 0.0) (Transformation|GetWorldRotation _sphere)) "None" false)
  (Variables|Default|Set上一帧世界位置 (Transformation|GetWorldLocation (Variables|Default|GetSphere))))

(event Collision|EventHit
  (params (MyComp :type Primitive%20Component%20Object%20Reference) (Other :type Actor%20Object%20Reference) (OtherComp :type Primitive%20Component%20Object%20Reference) (bSelfMoved :type Boolean) (HitLocation :type Vector :default "0, 0, 0") (HitNormal :type Vector :default "0, 0, 0") (NormalImpulse :type Vector :default "0, 0, 0") (Hit :type Hit%20Result%20Structure%20%28by%20ref%29))
  (Development|PrintString "命中1")
  (Variables|Default|Set击中位置 HitLocation)
  (Game|SpawnActorfromClass "/Game/BluePrints/hit_effect.hit_effect_C" (Math|Transform|MakeTransform (Variables|Default|Get击中位置) "0, 0, 0" "1.000000,1.000000,1.000000") "Undefined" "MultiplyWithRoot" 0 0))

(event EventTick
  (params (DeltaSeconds :type Float%20%28single-precision%29))
  (bind (_outhit _returnvalue) (Collision|LineTraceByChannel (Variables|Default|Get上一帧世界位置) (Transformation|GetWorldLocation (Variables|Default|GetSphere)) "TraceTypeQuery1" false 0 "Persistent"))
  (Variables|Default|Set上一帧世界位置 (Transformation|GetWorldLocation (Variables|Default|GetSphere)))
  (if _returnvalue
    (Variables|Default|Set击中位置 (.location _outhit))
    (Development|PrintString "命中2")
    (Game|SpawnActorfromClass "/Game/BluePrints/hit_effect.hit_effect_C" (Math|Transform|MakeTransform (Variables|Default|Get击中位置) "0, 0, 0" "1.000000,1.000000,1.000000") "Undefined" "MultiplyWithRoot" 0 0)))

(fn ConstructionScript)