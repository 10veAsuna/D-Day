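; BP_Soldier is a soldier Blueprint that drives movement-based camera shake for the first player's view.
; Every Tick calls a CameraShake event, which picks the Idle, Walk or Rush shake class from the soldier's speed, with Rush above a fixed threshold.
; The chosen shake is started again each frame on player controller 0, with no check for a change in movement state.
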(event Custom|CameraShake
  (bind _returnvalue (Game|GetPlayerController 0))
  ;[0.15 0.15 0.15 0.5] 相机抖动
  (if (<= (Math|Vector|VectorLength (Transformation|GetVelocity)) 0.0)
    (Game|Feedback|ClientStartCameraShake _returnvalue "/Game/BluePrints/CameraShake/BP_CameraShake_Idle.BP_CameraShake_Idle_C" 1.0 "CameraLocal" "0, 0, 0")
    (elif (> (Math|Vector|VectorLength (Transformation|GetVelocity)) 6e+02)
      (Game|Feedback|ClientStartCameraShake _returnvalue "/Game/BluePrints/CameraShake/BP_CameraShake_Rush.BP_CameraShake_Rush_C" 1.0 "CameraLocal" "0, 0, 0")
      (else
        (Game|Feedback|ClientStartCameraShake _returnvalue "/Game/BluePrints/CameraShake/BP_CameraShake_Walk.BP_CameraShake_Walk_C" 1.0 "CameraLocal" "0, 0, 0")))))

(event EventTick
  (params (DeltaSeconds :type Float%20%28single-precision%29))
  (CallFunction|CameraShake))

(fn ConstructionScript)