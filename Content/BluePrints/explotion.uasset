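; Reusable explosion actor that plays a Niagara effect and sound and damages BP_FriendAI and BP_Soldier actors.
; 启用 briefly enables three hurt boxes and calls 造成伤害, which applies a separate damage tier per box, stacking on overlaps.
; HurtBox1 is set to PhysicsOnly, unlike the others, so its overlap query likely finds nothing.
; After delayed effect shutdown Used is cleared; 禁用 also clears it and disables collision, but leaves Niagara visible.
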(event Custom|造成伤害
  (bind _hurtbox (Variables|Default|GetHurtBox))
  (bind _hurtbox1 (Variables|Default|GetHurtBox1))
  (bind _hurtbox2 (Variables|Default|GetHurtBox2))
  (Utilities|FlowControl|Sequence
    (:then_0
      (Utilities|FlowControl|Sequence
        (:then_0
          (for _array_element (Collision|GetOverlappingActors _hurtbox "/Game/AI/AIBluePrints/BP_FriendAI.BP_FriendAI_C" :!class /Script/Engine.PrimitiveComponent)
            (Game|Damage|ApplyDamage _array_element 6e+01 0 0)))
        (:then_1
          (for _array_element_2 (Collision|GetOverlappingActors _hurtbox "/Game/BluePrints/Character/BP_Soldier.BP_Soldier_C" :!class /Script/Engine.PrimitiveComponent)
            (Game|Damage|ApplyDamage _array_element_2 6e+01 0 0)))))
    (:then_1
      (Utilities|FlowControl|Sequence
        (:then_0
          (for _array_element_3 (Collision|GetOverlappingActors _hurtbox1 "/Game/AI/AIBluePrints/BP_FriendAI.BP_FriendAI_C" :!class /Script/Engine.PrimitiveComponent)
            (Game|Damage|ApplyDamage _array_element_3 25.0 0 0)))
        (:then_1
          (for _array_element_4 (Collision|GetOverlappingActors _hurtbox1 "/Game/BluePrints/Character/BP_Soldier.BP_Soldier_C" :!class /Script/Engine.PrimitiveComponent)
            (Game|Damage|ApplyDamage _array_element_4 25.0 0 0)))))
    (:then_2
      (Utilities|FlowControl|Sequence
        (:then_0
          (for _array_element_5 (Collision|GetOverlappingActors _hurtbox2 "/Game/AI/AIBluePrints/BP_FriendAI.BP_FriendAI_C" :!class /Script/Engine.PrimitiveComponent)
            (Game|Damage|ApplyDamage _array_element_5 15.0 0 0)))
        (:then_1
          (for _array_element_6 (Collision|GetOverlappingActors _hurtbox2 "/Game/BluePrints/Character/BP_Soldier.BP_Soldier_C" :!class /Script/Engine.PrimitiveComponent)
            (Game|Damage|ApplyDamage _array_element_6 15.0 0 0)))))))

(event Custom|启用
  (bind _niagara (Variables|Default|GetNiagara))
  (bind _niagara_2 (Variables|Default|GetNiagara))
  (Collision|SetCollisionEnabled (Variables|Default|GetHurtBox) "QueryAndPhysics")
  (Collision|SetCollisionEnabled (Variables|Default|GetHurtBox1) "PhysicsOnly")
  (Collision|SetCollisionEnabled (Variables|Default|GetHurtBox2) "QueryAndPhysics")
  (Transformation|AttachComponentToComponent _niagara (Variables|Default|GetDefaultSceneRoot) "None" "SnapToTarget" "SnapToTarget" "SnapToTarget" true)
  (Components|Activation|Activate _niagara false)
  (Rendering|SetVisibility _niagara true false)
  (Audio|PlaySoundatLocation "/Game/Sound/explotion2.explotion2" (Transformation|GetWorldLocation (Variables|Default|GetDefaultSceneRoot)) "0, 0, 0" 1.0 1.0 0.0 0 0 0 0)
  (CallFunction|造成伤害)
  (Utilities|FlowControl|Delay 0.2)
  (Collision|SetCollisionEnabled (Variables|Default|GetHurtBox) "NoCollision")
  (Collision|SetCollisionEnabled (Variables|Default|GetHurtBox1) "NoCollision")
  (Collision|SetCollisionEnabled (Variables|Default|GetHurtBox2) "NoCollision")
  (Utilities|FlowControl|Delay 4.5)
  (Components|Activation|Deactivate _niagara_2)
  (Rendering|SetVisibility _niagara_2 false false)
  (Variables|Default|Setused? false))

(event Custom|禁用
  (Collision|SetCollisionEnabled (Variables|Default|GetHurtBox) "NoCollision")
  (Collision|SetCollisionEnabled (Variables|Default|GetHurtBox1) "NoCollision")
  (Collision|SetCollisionEnabled (Variables|Default|GetHurtBox2) "NoCollision")
  (Rendering|SetVisibility (Variables|Default|GetNiagara) true false)
  (Variables|Default|Setused? false))

(fn ConstructionScript)