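; Mortar shell projectile that launches itself on spawn and explodes on impact.
; BeginPlay applies a physics impulse along the shell's rotation, scaled by mass and the initial-speed variable (初速).
; Impacts come from the Hit event or a per-tick Visibility trace between the sphere's previous and current positions, catching hits physics could miss.
; Either path spawns explosion FX and attenuated sound at the impact point, then destroys the actor.
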(event EventBeginPlay
  (bind _motar_shell (Variables|Default|GetMotar_shell))
  (Physics|AddImpulse (Variables|Default|GetMotar_shell) (Math|Vector|RotateVector (Math|Vector|MakeVector (* (* (Physics|GetMass _motar_shell) (Variables|Default|Get初速)) 5e+01) 0.0 0.0) (Transformation|GetWorldRotation _motar_shell)) "None" false)
  (Variables|Default|Set上一帧世界位置 (Transformation|GetWorldLocation (Variables|Default|GetSphere))))

(event Collision|EventHit
  (params (MyComp :type Primitive%20Component%20Object%20Reference) (Other :type Actor%20Object%20Reference) (OtherComp :type Primitive%20Component%20Object%20Reference) (bSelfMoved :type Boolean) (HitLocation :type Vector :default "0, 0, 0") (HitNormal :type Vector :default "0, 0, 0") (NormalImpulse :type Vector :default "0, 0, 0") (Hit :type Hit%20Result%20Structure%20%28by%20ref%29))
  (Development|PrintString "命中1")
  (Variables|Default|Set击中位置 HitLocation)
  (Niagara|SpawnSystematLocation "/Game/BluePrints/effect/FXS_explosion.FXS_explosion" (Variables|Default|Get击中位置))
  (Audio|PlaySoundatLocation "/Game/Sound/mortar_explosion.mortar_explosion" (Variables|Default|Get击中位置) "0, 0, 0" 1.0 1.0 0.0 "/Game/Sound/mortar_explosion1.mortar_explosion1" 0 0 0)
  (Actor|DestroyActor))

(event EventTick
  (params (DeltaSeconds :type Float%20%28single-precision%29))
  (bind _sphere (Variables|Default|GetSphere))
  (bind (_outhit _returnvalue) (Collision|LineTraceByChannel (Variables|Default|Get上一帧世界位置) (Transformation|GetWorldLocation _sphere) "TraceTypeQuery1" false 0 "None"))
  (Variables|Default|Set上一帧世界位置 (Transformation|GetWorldLocation _sphere))
  (if _returnvalue
    (Variables|Default|Set击中位置 (.location _outhit))
    (Development|PrintString "命中2")
    (Niagara|SpawnSystematLocation "/Game/BluePrints/effect/FXS_explosion.FXS_explosion" (Variables|Default|Get击中位置))
    (Audio|PlaySoundatLocation "/Game/Sound/mortar_explosion.mortar_explosion" (Variables|Default|Get击中位置) "0, 0, 0" 1.0 1.0 0.0 "/Game/Sound/mortar_explosion1.mortar_explosion1" 0 0 0)
    (Actor|DestroyActor)))

(fn ConstructionScript)