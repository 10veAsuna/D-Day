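; Actor that runs a recurring artillery bombardment, placing explosions at random ground points beneath its Box volume.
; BeginPlay waits briefly, then starts a looping timer and pre-spawns a small pool of disabled Explotion actors.
; Each timer tick, after a random delay, claims the first unused pooled actor, moves it to a downward trace hit from a random point in the box and enables it.
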(event Custom|炮击
  (Utilities|FlowControl|Delay (Math|Random|RandomFloatinRange 0.0 1.5))
  (CallFunction|生成炮击))

(event Custom|生成炮击
  (bind _box (Variables|Default|GetBox))
  (bind (_origin _boxextent) (Collision|GetComponentBounds _box))
  (bind _array_element (Utilities|Array|ForEachLoopwithBreak (Variables|Default|GetExplotionPool) :!label _label)
    (:LoopBody
      (bind _output_get (Variables|Default|SetArray%20Element _array_element))
      (if (Variables|/Game/BluePrints/explotion.explotion_C|Getused? _output_get)
        (Development|PrintString "go on")
        (else
          (Utilities|FlowControl|Sequence
            (:then_0
              (bind _output_get_2 (Variables|Default|Setlocation (Math|Random|RandomPointinBoundingBox _origin _boxextent)))
              (bind _outhit (Collision|LineTraceByChannel _output_get_2 (Math|Vector|MakeVector (.x (Variables|Default|Getlocation)) (.y (Variables|Default|Getlocation)) (- (.z (Variables|Default|Getlocation)) 999999.0)) "TraceTypeQuery1" false 0 "None"))
              (Variables|/Game/BluePrints/explotion.explotion_C|Setused? (Variables|Default|GetArray%20Element) true)
              (Transformation|SetWorldLocation (Variables|/Game/BluePrints/explotion.explotion_C|GetDefaultSceneRoot (Variables|Default|GetArray%20Element)) (.location _outhit) false false)
              (Default|启用 (Variables|Default|GetArray%20Element)))
            (:then_1
              (goto _label Break))))))
    (:Completed
      (Development|PrintString "full"))))

(event EventBeginPlay
  (Utilities|FlowControl|Delay 3.0)
  (Utilities|Time|SetTimerbyEvent (delegate Custom|炮击) 1.0 true)
  (for _index (range 0 4)
    (bind _returnvalue (Game|SpawnActorfromClass "/Game/BluePrints/explotion.explotion_C" (Math|Transform|MakeTransform "0, 0, 0" "0, 0, 0" "1.000000,1.000000,1.000000") "Undefined" "MultiplyWithRoot" 0 0))
    (Default|禁用 _returnvalue)
    (Utilities|Array|Add (Variables|Default|GetExplotionPool) _returnvalue))
  (Development|PrintString "Hello"))

(fn ConstructionScript)