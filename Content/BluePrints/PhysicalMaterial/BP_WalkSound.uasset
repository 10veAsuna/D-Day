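; BP_WalkSound is an animation notify that plays a surface-dependent footstep sound at the owning actor's location.
; When it fires, it traces 200 units straight down from that location on the Visibility channel and reads the surface type of the hit.
; Dirt, Grass and Water each play their own fixed sound; no other surface is handled.
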(fn ReceivedNotify
  (params (mesh :type Actor%20Component%20Object%20Reference))
  (bind _actorlocation (LocalVariables|GetactorLocation))
  (Utilities|IsValid (Components|GetOwner mesh)
    (:Is%20Valid
      (bind (_outhit _returnvalue) (Collision|LineTraceByChannel _actorlocation (- _actorlocation "0.000000,0.000000,200.000000") "TraceTypeQuery1" false 0 "None"))
      (if _returnvalue
        (switch Utilities|FlowControl|Switch|SwitchonEPhysicalSurface (Collision|GetSurfaceType _outhit)
          (:SurfaceType1
            (Audio|PlaySoundatLocation "/Game/sucai/Footstep_Sounds_Pro/Wavs/Dirt_footsteps/Dirt_footstep_1.Dirt_footstep_1" (LocalVariables|GetactorLocation) "0, 0, 0" 1.0 1.0 0.0 0 0 0 0))
          (:SurfaceType2
            (Audio|PlaySoundatLocation "/Game/Sound/Grass_footstep_2.Grass_footstep_2" (LocalVariables|GetactorLocation) "0, 0, 0" 1.0 1.0 0.0 0 0 0 0))
          (:SurfaceType3
            (Audio|PlaySoundatLocation "/Game/sucai/Footstep_Sounds_Pro/Wavs/Water_footsteps/Water_footstep_2.Water_footstep_2" (LocalVariables|GetactorLocation) "0, 0, 0" 1.0 1.0 0.0 0 0 0 0)))
        (return 0)))))