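; Player controller for a soldier shooter, handling Enhanced Input for movement, stance, camera switching, weapons, pause and debug death UI.
; An Action state sets walk speed; weapon swaps re-attach guns between back and hand sockets, with timer-driven Thompson and single-shot Garand fire.
; Aiming blends to a camera spawned on the weapon socket, and a per-tick sphere trace shows pickup prompts.
; It also possesses mortars by swapping mapping contexts and respawns the soldier.
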(event Custom|重新部署
  (bind _returnvalue (Game|GetPlayerController 0))
  (bind _dieui (Variables|Default|Getdieui))
  ;[0.15 0.15 0.15 0.5] 重新部署
  (bind _outactors (Actor|GetAllActorsOfClass "/Game/BluePrints/testbp/spawn.spawn_C"))
  (Development|PrintString "respawn")
  (if (> (Utilities|Array|Length _outactors) 0)
    (Development|PrintString "1")
    (Widget|RemovefromParent _dieui)
    (Development|PrintString "yichu")
    (Actor|DestroyActor (Pawn|GetControlledPawn))
    (bind _returnvalue_2 (Actor|GetActorOfClass "/Game/BluePrints/testbp/spawn.spawn_C"))
    (bind _returnvalue_3 (Game|SpawnActorfromClass "/Game/BluePrints/Character/BP_Soldier.BP_Soldier_C" (Transformation|GetActorTransform _returnvalue_2) "AdjustIfPossibleButAlwaysSpawn" "MultiplyWithRoot" 0 0))
    (bind _output_get (Variables|Default|SetBpSoldier _returnvalue_3))
    (Pawn|Possess _returnvalue _output_get)
    (Input|SetInputModeGameOnly _returnvalue false)
    (Variables|/Script/Engine.PlayerController|SetbShowMouseCursor _returnvalue false)
    (else
      (Development|PrintString "0")
      (Widget|RemovefromParent _dieui)
      (Development|PrintString "yichu")
      (Actor|DestroyActor (Pawn|GetControlledPawn))
      (bind _returnvalue_4 (Actor|GetActorOfClass "/Script/Engine.PlayerStart"))
      (bind _returnvalue_5 (Game|SpawnActorfromClass "/Game/BluePrints/Character/BP_Soldier.BP_Soldier_C" (Transformation|GetActorTransform _returnvalue_4) "AdjustIfPossibleButAlwaysSpawn" "MultiplyWithRoot" 0 0))
      (Pawn|Possess _returnvalue _returnvalue_5)
      (Input|SetInputModeGameOnly _returnvalue false)
      (Variables|/Script/Engine.PlayerController|SetbShowMouseCursor _returnvalue false))))

(event Custom|Interact
  (bind _interact1 (Variables|Default|GetInteract1))
  ;[0.15 0.15 0.15 0.5] 按F拾取
  (bind (_outhit _returnvalue) (CallFunction|RangeDetectionOfPicking))
  (if _returnvalue
    (bind _output_get (Variables|Default|SetHit%20Actor (.HitActor (Collision|BreakHitResult _outhit))))
    (if (Actor|ActorHasTag _output_get "Weapon")
      (switch Utilities|FlowControl|Switch|SwitchonENUM_Arm (Variables|Default|GetWeapon%20Attribute%20Weapon%20Arm)
        (:NewEnumerator0
          (UserInterface|Viewport|AddtoViewport (Variables|Default|GetInteract1) 0))
        (:NewEnumerator1
          (if (stale _output_get_2) :!label _label
            (Utilities|FlowControl|DoOnce false
              (:Completed
                (Development|PrintString (Utilities|String|EnumtoString (Variables|Default|GetWeapon%20Attribute%20Weapon%20Arm)))
                (Widget|RemovefromParent _interact1)))))
        (:NewEnumerator2
          (goto _label))))
    (else
      (Utilities|IsValid _interact1
        (:Is%20Valid
          (bind _output_get_2 (Variables|Default|Setvalid true)))))))

(event Custom|GetWeaponToHand
  (params (目标 :type Actor%20Object%20Reference))
  ;[0.15 0.15 0.15 0.5] 换枪
  (Utilities|GetAllWeapontoBack
    (:真
      (bind _returnvalue (Utilities|Handweapon 目标))
      (if _returnvalue
        (bind _asset (Class|APIEquip|GetEquippedWeaponDataAsset(Message) 目标))
        (bind _output_get (Variables|Default|SetEquippedWeapon (.weapontype (Variables|/Game/BluePrints/weapon/BP_Weapon.BP_Weapon_C|GetWeaponAttri _asset))))
        (Variables|/Game/Animation/ABP_FirstPerson.ABP_FirstPerson_C|SetEquippedWeapon (Variables|Default|GetAs%20ABP%20First%20Person) _output_get)))))

(event Custom|ThompsonFire
  ;[0.15 0.15 0.15 0.5] 开火
  (bind _equippedthompson (Variables|/Game/BluePrints/Character/BP_Soldier.BP_Soldier_C|GetEquippedThompson (Variables|Default|GetAs%20BP%20Soldier))
    (:then
      (Class|APIEquip|Fire(Message) _equippedthompson))
    (:else)))

(event Input|EnhancedActionEvents|EnhancedInputActionIA_PickUp
  (params (ActionValue :type Boolean) (ElapsedSeconds :type Float%20%28double-precision%29) (TriggeredSeconds :type Float%20%28double-precision%29) (InputAction :type Input%20Action%20Object%20Reference :default "/Game/Input/IA_PickUp.IA_PickUp"))
  (bind _returnvalue (PlayerController|LocalPlayerSubsystems|GetEnhancedInputLocalPlayerSubsystem))
  ;[0.15 0.15 0.15 0.5] 操控迫击炮
  (:Started
    (Development|PrintString "Hello0")
    (bind _returnvalue_2 (Actor|GetActorOfClass "/Game/BluePrints/Character/BP_Soldier.BP_Soldier_C"))
    (for _array_element (Collision|GetOverlappingActors _returnvalue_2 "/Game/BluePrints/mortar.mortar_C" :!class /Script/Engine.Actor)
      (Utilities|IsValid _array_element
        (:Is%20Valid
          (bind _asmortar (Utilities|Casting|CastTomortar _array_element)
            (:then
              (Input|RemoveMappingContext _returnvalue "/Game/Input/IMC_My.IMC_My" "(bIgnoreAllPressedKeysUntilRelease=True,bForceImmediately=False,bNotifyUserSettings=False)")
              (Input|AddMappingContext _returnvalue "/Game/Input/IMC_mortar.IMC_mortar" 0 "(bIgnoreAllPressedKeysUntilRelease=True,bForceImmediately=False,bNotifyUserSettings=False)")
              (Pawn|Possess _asmortar)
              (bind _returnvalue_3 (UserInterface|CreateWidget "/Game/UI/WBP_mortar.WBP_mortar_C"))
              (bind _output_get (Variables|Default|SetMortarUI _returnvalue_3))
              (UserInterface|Viewport|AddtoViewport _output_get 0)
              (bind _returnvalue_4 (Actor|GetActorOfClass "/Game/BluePrints/Character/BP_Soldier.BP_Soldier_C"))
              (Rendering|SetActorHiddenInGame _returnvalue_4 true))
            (:CastFailed
              (Development|PrintString "Hello3"))))
        (:Is%20Not%20Valid
          (Development|PrintString "Hello2"))))))

(event Input|EnhancedActionEvents|EnhancedInputActionIAmortar_out
  (params (ActionValue :type Boolean) (ElapsedSeconds :type Float%20%28double-precision%29) (TriggeredSeconds :type Float%20%28double-precision%29) (InputAction :type Input%20Action%20Object%20Reference :default "/Game/Input/IA_mortar/IAmortar_out.IAmortar_out"))
  (bind _returnvalue (PlayerController|LocalPlayerSubsystems|GetEnhancedInputLocalPlayerSubsystem))
  ;[0.15 0.15 0.15 0.5] 离开迫击炮
  (:Started
    (Input|RemoveMappingContext _returnvalue "/Game/Input/IMC_mortar.IMC_mortar" "(bIgnoreAllPressedKeysUntilRelease=True,bForceImmediately=False,bNotifyUserSettings=False)")
    (Input|AddMappingContext _returnvalue "/Game/Input/IMC_My.IMC_My" 0 "(bIgnoreAllPressedKeysUntilRelease=True,bForceImmediately=False,bNotifyUserSettings=False)")
    (bind _returnvalue_2 (Actor|GetActorOfClass "/Game/BluePrints/Character/BP_Soldier.BP_Soldier_C"))
    (Pawn|Possess (Game|GetPlayerController 0) _returnvalue_2)
    (Rendering|SetActorHiddenInGame _returnvalue_2 false)
    (Widget|RemovefromParent (Variables|Default|GetMortarUI))))

(event Input|EnhancedActionEvents|EnhancedInputActionIA_Jump
  (params (ActionValue :type Boolean) (ElapsedSeconds :type Float%20%28double-precision%29) (TriggeredSeconds :type Float%20%28double-precision%29) (InputAction :type Input%20Action%20Object%20Reference :default "/Game/Input/IA_Jump.IA_Jump"))
  (bind _returnvalue (Game|GetPlayerCharacter 0))
  ;[0.15 0.15 0.15 0.5] 跳跃
  (:Started
    (switch Utilities|FlowControl|Switch|SwitchonENUM_Action (Variables|Default|GetAction)
      (:NewEnumerator0
        _)
      (:NewEnumerator1
        _))
    (Character|Jump _returnvalue))
  (:Completed
    (Character|StopJumping _returnvalue)))

(event Input|EnhancedActionEvents|EnhancedInputActionIA_Crouch
  (params (ActionValue :type Boolean) (ElapsedSeconds :type Float%20%28double-precision%29) (TriggeredSeconds :type Float%20%28double-precision%29) (InputAction :type Input%20Action%20Object%20Reference :default "/Game/Input/IA_Crouch.IA_Crouch"))
  ;[0.15 0.15 0.15 0.5] 蹲
  (:Ongoing
    (switch Utilities|FlowControl|Switch|SwitchonENUM_Action (Variables|Default|GetAction)
      (:NewEnumerator0
        (Utilities|ChangeSpeed "NewEnumerator3" :!label _label))
      (:NewEnumerator1
        (goto _label))
      (:NewEnumerator5
        (Utilities|ChangeSpeed "NewEnumerator7" :!label _label_2))
      (:NewEnumerator6
        (goto _label_2)))
    (bind _asbp_soldier (Utilities|Casting|CastToBP_Soldier (Pawn|GetControlledPawn)))
    (Character|Crouch _asbp_soldier)
    (Variables|Default|SetIsCrouch true))
  (:Completed
    (switch Utilities|FlowControl|Switch|SwitchonENUM_Action (Variables|Default|GetAction)
      (:NewEnumerator3
        (Utilities|ChangeSpeed "NewEnumerator0"))
      (:NewEnumerator7
        (Utilities|ChangeSpeed "NewEnumerator5")))
    (Character|UnCrouch _asbp_soldier)
    (Variables|Default|SetIsCrouch false)))

(event Input|EnhancedActionEvents|EnhancedInputActionIA_Rush
  (params (ActionValue :type Boolean) (ElapsedSeconds :type Float%20%28double-precision%29) (TriggeredSeconds :type Float%20%28double-precision%29) (InputAction :type Input%20Action%20Object%20Reference :default "/Game/Input/IA_Rush.IA_Rush"))
  (bind _action (Variables|Default|GetAction))
  ;[0.15 0.15 0.15 0.5] 加速跑
  (:Triggered
    (if (not (Variables|/Game/BluePrints/Character/BP_Soldier.BP_Soldier_C|GetIsAiming (Variables|Default|GetAs%20BP%20Soldier)))
      (switch Utilities|FlowControl|Switch|SwitchonENUM_Action _action
        (:NewEnumerator0
          (Utilities|ChangeSpeed "NewEnumerator1")
          (if true
            (bind _as角色 (Utilities|Casting|CastToCharacter (Pawn|GetControlledPawn)))
            (Variables|/Script/Engine.CharacterMovementComponent|SetMaxWalkSpeed (Variables|/Script/Engine.Character|GetCharacterMovement _as角色) 6e+02)
            (else
              (bind _as角色_2 (Utilities|Casting|CastToCharacter (Pawn|GetControlledPawn) :!label _label))
              (Variables|/Script/Engine.CharacterMovementComponent|SetMaxWalkSpeed (Variables|/Script/Engine.Character|GetCharacterMovement _as角色_2) 3e+02)))))))
  (:Completed
    (switch Utilities|FlowControl|Switch|SwitchonENUM_Action _action
      (:NewEnumerator1
        (Utilities|ChangeSpeed "NewEnumerator0")
        (goto _label)))))

(event Input|EnhancedActionEvents|EnhancedInputActionIA_SwitchCamera
  (params (ActionValue :type Boolean) (ElapsedSeconds :type Float%20%28double-precision%29) (TriggeredSeconds :type Float%20%28double-precision%29) (InputAction :type Input%20Action%20Object%20Reference :default "/Game/Input/IA_SwitchCamera.IA_SwitchCamera"))
  ;[0.15 0.15 0.15 0.5] 切换视角
  (:Started
    (bind _asbp_soldier (Utilities|Casting|CastToBP_Soldier (Pawn|GetControlledPawn)))
    (Utilities|FlowControl|FlipFlop
      (:A
        (Components|Activation|SetActive (Variables|/Game/BluePrints/Character/BP_Soldier.BP_Soldier_C|GetFCamera _asbp_soldier) true false)
        (Components|Activation|SetActive (Variables|/Game/BluePrints/Character/BP_Soldier.BP_Soldier_C|GetTCamera _asbp_soldier) false false))
      (:B
        (Components|Activation|SetActive (Variables|/Game/BluePrints/Character/BP_Soldier.BP_Soldier_C|GetTCamera _asbp_soldier) true false)
        (Components|Activation|SetActive (Variables|/Game/BluePrints/Character/BP_Soldier.BP_Soldier_C|GetFCamera _asbp_soldier) false false)))))

(event Input|EnhancedActionEvents|EnhancedInputActionIA_3
  (params (ActionValue :type Boolean) (ElapsedSeconds :type Float%20%28double-precision%29) (TriggeredSeconds :type Float%20%28double-precision%29) (InputAction :type Input%20Action%20Object%20Reference :default "/Game/Input/IA_3.IA_3"))
  ;[0.15 0.15 0.15 0.5] 换枪
  (:Started
    (if (not (Variables|/Game/BluePrints/Character/BP_Soldier.BP_Soldier_C|GetIsAiming (Variables|Default|GetAs%20BP%20Soldier)))
      (if (Variables|/Game/Animation/ABP_FirstPerson.ABP_FirstPerson_C|GetisArmed (Variables|Default|GetAs%20ABP%20First%20Person))
        (Variables|/Game/Animation/ABP_FirstPerson.ABP_FirstPerson_C|SetisArmed (Variables|Default|GetAs%20ABP%20First%20Person) false)
        (if (not (Variables|/Game/Animation/ABP_FirstPerson.ABP_FirstPerson_C|GetisArmed (Variables|Default|GetAs%20ABP%20First%20Person)))
          (Utilities|GetAllWeapontoBack
            (:真
              (Transformation|AttachComponentToComponent (Variables|/Game/BluePrints/Character/BP_Soldier.BP_Soldier_C|GetEquippedGarand (Variables|Default|GetAs%20BP%20Soldier)) (Variables|/Script/Engine.Character|GetMesh (Variables|Default|GetAs%20BP%20Soldier)) "weapon" "SnapToTarget" "SnapToTarget" "SnapToTarget" true)
              (Variables|Default|SetEquippedWeapon "NewEnumerator2"))))))))

(event Input|EnhancedActionEvents|EnhancedInputActionIA_Pause
  (params (ActionValue :type Boolean) (ElapsedSeconds :type Float%20%28double-precision%29) (TriggeredSeconds :type Float%20%28double-precision%29) (InputAction :type Input%20Action%20Object%20Reference :default "/Game/Input/IA_Pause.IA_Pause"))
  ;[0.15 0.15 0.15 0.5] 暂停
  (:Started
    (Game|SetGamePaused true)
    (Input|SetInputModeUIOnly self 0 "DoNotLock" false)
    (Variables|Default|SetbShowMouseCursor true)
    (bind _returnvalue (UserInterface|CreateWidget "/Game/UI/WBP_Pause.WBP_Pause_C"))
    (UserInterface|Viewport|AddtoViewport _returnvalue 0)))

(event Input|EnhancedActionEvents|EnhancedInputActionIA_2
  (params (ActionValue :type Boolean) (ElapsedSeconds :type Float%20%28double-precision%29) (TriggeredSeconds :type Float%20%28double-precision%29) (InputAction :type Input%20Action%20Object%20Reference :default "/Game/Input/IA_2.IA_2"))
  ;[0.15 0.15 0.15 0.5] 换枪
  (:Started
    (if (not (Variables|/Game/BluePrints/Character/BP_Soldier.BP_Soldier_C|GetIsAiming (Variables|Default|GetAs%20BP%20Soldier)))
      (if (Variables|/Game/Animation/ABP_FirstPerson.ABP_FirstPerson_C|GetisArmed (Variables|Default|GetAs%20ABP%20First%20Person))
        (bind _equippedthompson (Variables|/Game/BluePrints/Character/BP_Soldier.BP_Soldier_C|GetEquippedThompson (Variables|Default|GetAs%20BP%20Soldier) :!label _label)
          (:then
            (CallFunction|GetWeapontoHand _equippedthompson)
            (Variables|Default|SetEquippedWeapon "NewEnumerator0"))
          (:else))
        (else
          (Variables|/Game/Animation/ABP_FirstPerson.ABP_FirstPerson_C|SetisArmed (Variables|Default|GetAs%20ABP%20First%20Person) true)
          (if (Variables|/Game/Animation/ABP_FirstPerson.ABP_FirstPerson_C|GetisArmed (Variables|Default|GetAs%20ABP%20First%20Person))
            (goto _label)))))))

(event Input|EnhancedActionEvents|EnhancedInputActionIA_Camera
  (params (ActionValue :type Vector%202D%20Structure) (ElapsedSeconds :type Float%20%28double-precision%29) (TriggeredSeconds :type Float%20%28double-precision%29) (InputAction :type Input%20Action%20Object%20Reference :default "/Game/Input/IA_Camera.IA_Camera"))
  ;[0.15 0.15 0.15 0.5] 移动视角
  (Class|PlayerController|AddYawInput (* (Variables|Default|GetSensitivity) (.x ActionValue)))
  (Class|PlayerController|AddPitchInput (* (.y ActionValue) (Variables|Default|GetSensitivity))))

(event Input|EnhancedActionEvents|EnhancedInputActionIA_1
  (params (ActionValue :type Boolean) (ElapsedSeconds :type Float%20%28double-precision%29) (TriggeredSeconds :type Float%20%28double-precision%29) (InputAction :type Input%20Action%20Object%20Reference :default "/Game/Input/IA_1.IA_1"))
  ;[0.15 0.15 0.15 0.5] 换枪
  (:Started
    (if (not (Variables|/Game/BluePrints/Character/BP_Soldier.BP_Soldier_C|GetIsAiming (Variables|Default|GetAs%20BP%20Soldier)))
      (if (Variables|/Game/Animation/ABP_FirstPerson.ABP_FirstPerson_C|GetisArmed (Variables|Default|GetAs%20ABP%20First%20Person))
        (bind _equippedgarand (Variables|/Game/BluePrints/Character/BP_Soldier.BP_Soldier_C|GetEquippedGarand (Variables|Default|GetAs%20BP%20Soldier) :!label _label)
          (:then
            (CallFunction|GetWeapontoHand _equippedgarand)
            (Variables|Default|SetEquippedWeapon "NewEnumerator1")
            (Class|APIUI|ShowBulletNumber(Message) (Variables|Default|GetBulletUI))
            (Class|APIUI|UpdateBulletNumber(Message) (Variables|Default|GetBulletUI) 0 (Utilities|Select :Index "NewEnumerator0" :NewEnumerator0 0 :NewEnumerator1 0 :NewEnumerator2 0)))
          (:else))
        (else
          (Variables|/Game/Animation/ABP_FirstPerson.ABP_FirstPerson_C|SetisArmed (Variables|Default|GetAs%20ABP%20First%20Person) true)
          (if (Variables|/Game/Animation/ABP_FirstPerson.ABP_FirstPerson_C|GetisArmed (Variables|Default|GetAs%20ABP%20First%20Person))
            (goto _label)))))))

(event Input|EnhancedActionEvents|EnhancedInputActionIA_Aim
  (params (ActionValue :type Boolean) (ElapsedSeconds :type Float%20%28double-precision%29) (TriggeredSeconds :type Float%20%28double-precision%29) (InputAction :type Input%20Action%20Object%20Reference :default "/Game/Input/IA_Aim.IA_Aim"))
  (bind _as_bp_soldier (Variables|Default|GetAs%20BP%20Soldier))
  (:Started
    (Utilities|FlowControl|FlipFlop
      (:A
        (if (Variables|/Game/Animation/ABP_FirstPerson.ABP_FirstPerson_C|GetisArmed (Variables|Default|GetAs%20ABP%20First%20Person))
          (Variables|/Game/BluePrints/Character/BP_Soldier.BP_Soldier_C|SetIsAiming (Variables|Default|GetAs%20BP%20Soldier) true)
          (bind _returnvalue (Game|SpawnActorfromClass "/Game/BluePrints/weapon/BP_Camera.BP_Camera_C" (Math|Transform|MakeTransform "0, 0, 0" "0, 0, 0" "1.000000,1.000000,1.000000") "AdjustIfPossibleButAlwaysSpawn" "MultiplyWithRoot" 0 0))
          (switch Utilities|FlowControl|Switch|SwitchonENUM_WeaponType (Variables|Default|GetEquippedWeapon)
            (:NewEnumerator0
              (Transformation|AttachComponentToComponent _returnvalue (Variables|/Game/BluePrints/weapon/BP_EquippedWeapon.BP_EquippedWeapon_C|GetSkeletalMesh (Variables|/Game/BluePrints/Character/BP_Soldier.BP_Soldier_C|GetEquippedThompson _as_bp_soldier)) "ThompsonCamera" "SnapToTarget" "SnapToTarget" "SnapToTarget" true))
            (:NewEnumerator1
              (Transformation|AttachComponentToComponent _returnvalue (Variables|/Game/BluePrints/weapon/BP_EquippedWeapon.BP_EquippedWeapon_C|GetSkeletalMesh (Variables|/Game/BluePrints/Character/BP_Soldier.BP_Soldier_C|GetEquippedGarand _as_bp_soldier)) "GarandCamera" "SnapToTarget" "SnapToTarget" "SnapToTarget" true)))
          (Game|Player|SetViewTargetwithBlend _returnvalue 0.3 "VTBlend_Cubic" 0.0 false)
          (Camera|SetFieldOfView (Variables|/Game/BluePrints/weapon/BP_Camera.BP_Camera_C|GetCamera _returnvalue) 5e+01)))
      (:B
        (if (Variables|/Game/Animation/ABP_FirstPerson.ABP_FirstPerson_C|GetisArmed (Variables|Default|GetAs%20ABP%20First%20Person))
          (Variables|/Game/BluePrints/Character/BP_Soldier.BP_Soldier_C|SetIsAiming (Variables|Default|GetAs%20BP%20Soldier) false)
          (Actor|DestroyActor _returnvalue)
          (Game|Player|SetViewTargetwithBlend (Variables|Default|GetAs%20BP%20Soldier) 0.3 "VTBlend_Cubic" 0.0 false))))))

(event Input|EnhancedActionEvents|EnhancedInputActionIA_Fire
  (params (ActionValue :type Boolean) (ElapsedSeconds :type Float%20%28double-precision%29) (TriggeredSeconds :type Float%20%28double-precision%29) (InputAction :type Input%20Action%20Object%20Reference :default "/Game/Input/IA_Fire.IA_Fire"))
  (bind _as_bp_soldier (Variables|Default|GetAs%20BP%20Soldier))
  ;[0.15 0.15 0.15 0.5] 开火
  (:Triggered
    (switch Utilities|FlowControl|Switch|SwitchonENUM_WeaponType (Variables|Default|GetEquippedWeapon)
      (:NewEnumerator0
        (bind _equippedthompson (Variables|/Game/BluePrints/Character/BP_Soldier.BP_Soldier_C|GetEquippedThompson _as_bp_soldier)
          (:then
            (bind _returnvalue (Utilities|Time|SetTimerbyEvent (delegate Custom|ThompsonFire) (.weaponfiringrate (Variables|/Game/BluePrints/weapon/BP_Weapon.BP_Weapon_C|GetWeaponAttri (Variables|/Game/BluePrints/weapon/BP_EquippedWeapon.BP_EquippedWeapon_C|GetWeaponDataAsset _equippedthompson))) true))
            (Variables|Default|Settimer _returnvalue))
          (:else)))))
  (:Started
    (switch Utilities|FlowControl|Switch|SwitchonENUM_WeaponType (Variables|Default|GetEquippedWeapon)
      (:NewEnumerator1
        (Class|APIEquip|Fire(Message) (Variables|/Game/BluePrints/Character/BP_Soldier.BP_Soldier_C|GetEquippedGarand _as_bp_soldier)))))
  (:Completed
    (switch Utilities|FlowControl|Switch|SwitchonENUM_WeaponType (Variables|Default|GetEquippedWeapon)
      (:NewEnumerator0
        (Utilities|Time|ClearandInvalidateTimerbyHandle (Variables|Default|Gettimer))))))

(event Input|EnhancedActionEvents|EnhancedInputActionIA_Movement
  (params (ActionValue :type Vector%202D%20Structure) (ElapsedSeconds :type Float%20%28double-precision%29) (TriggeredSeconds :type Float%20%28double-precision%29) (InputAction :type Input%20Action%20Object%20Reference :default "/Game/Input/IA_Movement.IA_Movement"))
  (bind _returnvalue (Pawn|GetControlledPawn))
  (bind _returnvalue_2 (Transformation|GetActorRotation _returnvalue))
  ;[0.15 0.15 0.15 0.5] 移动
  (Pawn|Input|AddMovementInput _returnvalue (Math|Vector|GetForwardVector (Math|Rotator|MakeRotator 0.0 0.0 (.yaw _returnvalue_2))) (.x ActionValue) false)
  (Pawn|Input|AddMovementInput _returnvalue (Math|Vector|GetRightVector (Math|Rotator|MakeRotator 0.0 0.0 (.yaw _returnvalue_2))) (.y ActionValue) false))

(event EventBeginPlay
  (Utilities|FlowControl|Sequence
    (:then_0
      (bind _asbp_soldier (Utilities|Casting|CastToBP_Soldier (Game|GetPlayerCharacter 0)))
      (Variables|Default|SetAs%20BP%20Soldier _asbp_soldier)
      (CallFunction|AddEnhancedInput)
      (bind _returnvalue (UserInterface|CreateWidget "/Game/UI/die.die_C"))
      (Variables|Default|Setdieui _returnvalue)
      (bind _returnvalue_2 (UserInterface|CreateWidget "/Game/UI/WBP_Interact.WBP_Interact_C"))
      (Variables|Default|SetInteract1 _returnvalue_2)
      (bind _returnvalue_3 (UserInterface|CreateWidget "/Game/UI/WBP_total.WBP_total_C"))
      (Variables|Default|SetTotalUI _returnvalue_3)
      (bind _returnvalue_4 (UserInterface|CreateWidget "/Game/UI/WBP_Bullet.WBP_Bullet_C"))
      (Variables|Default|SetBulletUI _returnvalue_4))
    (:then_1
      (bind _asabp_first_person (Utilities|Casting|CastToABP_FirstPerson (Components|SkeletalMesh|GetAnimInstance (Variables|/Script/Engine.Character|GetMesh (Variables|Default|GetAs%20BP%20Soldier)))))
      (Variables|Default|SetAs%20ABP%20First%20Person _asabp_first_person))))

(event EventTick
  (params (DeltaSeconds :type Float%20%28single-precision%29))
  (CallFunction|Interact))

(event Input|KeyboardEvents|9
  (params (Key :type Key%20Structure :default "None"))
  (bind _returnvalue (Game|GetPlayerController 0))
  ;[0.15 0.15 0.15 0.5] 死亡测试
  (:Pressed
    (UserInterface|Viewport|AddtoViewport (Variables|Default|Getdieui) 0)
    (Input|SetInputModeGameandUI _returnvalue 0 "DoNotLock" true false)
    (Variables|/Script/Engine.PlayerController|SetbShowMouseCursor _returnvalue true)))

(event Input|KeyboardEvents|T
  (params (Key :type Key%20Structure :default "None"))
  (bind _totalui (Variables|Default|GetTotalUI))
  (:Pressed
    (Utilities|FlowControl|FlipFlop
      (:A
        (UserInterface|Viewport|AddtoViewport _totalui 0)
        (Utilities|FlowControl|Delay 3.0)
        (Utilities|IsValid _totalui
          (:Is%20Valid
            (Widget|RemovefromParent _totalui))))
      (:B
        (Utilities|IsValid _totalui
          (:Is%20Valid
            (Widget|RemovefromParent _totalui)))))))

(fn ConstructionScript)

(fn AddEnhancedInput
  (bind _self self)
  (bind _returnvalue (PlayerController|LocalPlayerSubsystems|GetEnhancedInputLocalPlayerSubsystem _self))
  (Utilities|IsValid _returnvalue
    (:Is%20Valid
      (Input|AddMappingContext _returnvalue "/Game/Input/IMC_My.IMC_My" 0 "(bIgnoreAllPressedKeysUntilRelease=True,bForceImmediately=False,bNotifyUserSettings=False)"))))

(fn RangeDetectionOfPicking
  (bind _returnvalue (Game|GetPlayerCameraManager 0))
  (bind _returnvalue_2 (Transformation|GetActorLocation _returnvalue))
  (bind (_outhit _returnvalue_3) (Collision|SphereTraceByChannel _returnvalue_2 (+ _returnvalue_2 (* (Transformation|GetActorForwardVector _returnvalue) "350.000000,350.000000,350.000000")) 1e+01 "TraceTypeQuery3" false 0 "None"))
  (return _outhit _returnvalue_3))