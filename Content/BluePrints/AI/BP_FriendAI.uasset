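; Friendly AI character that appears as a US WWII paratrooper and wanders the level.
; On BeginPlay, a randomized MultiGate picks one of four paratrooper skeletal meshes, then patrolling starts.
; Patrol uses AI MoveTo toward a random reachable point near the current location and restarts on success or failure, so the wander area drifts with the character.
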(event Custom|GoOnPatrol
  (AI|AIMoveTo 0 (.RandomLocation (AI|Navigation|GetRandomReachablePointinRadius (Transformation|GetActorLocation) 5e+02 0 0)) 0 5.0 false
    (:OnSuccess
      _)
    (:OnFail
      _))
  (CallFunction|GoonPatrol))

(event Custom|RandomMesh
  (bind _mesh (Variables|Character|GetMesh))
  (Utilities|FlowControl|MultiGate true false (Math|Random|RandomIntegerinRange 0 3)
    (:Out%200
      (Components|SkeletalMesh|SetSkeletalMeshAsset _mesh "/Game/AlliedMilitaryFigureModel/Meshes/SK_WWII_US_Paratrooper_no_helmet.SK_WWII_US_Paratrooper_no_helmet"))
    (:Out%201
      (Components|SkeletalMesh|SetSkeletalMeshAsset _mesh "/Game/AlliedMilitaryFigureModel/Meshes/SK_WWII_US_Paratrooper_no_helmet_w_equipment.SK_WWII_US_Paratrooper_no_helmet_w_equipment"))
    (:Out%202
      (Components|SkeletalMesh|SetSkeletalMeshAsset _mesh "/Game/AlliedMilitaryFigureModel/Meshes/SK_WWII_US_Paratrooper_simple.SK_WWII_US_Paratrooper_simple"))
    (:Out%203
      (Components|SkeletalMesh|SetSkeletalMeshAsset _mesh "/Game/AlliedMilitaryFigureModel/Meshes/SK_WWII_US_Paratrooper_simpleB.SK_WWII_US_Paratrooper_simpleB"))))

(event EventBeginPlay
  (CallFunction|RandomMesh)
  (CallFunction|GoonPatrol))

(fn ConstructionScript)