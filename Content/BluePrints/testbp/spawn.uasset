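; Spawner actor that keeps a population of up to 50 BP_FriendAI actors around its own location.
; A looping 10-second timer started on BeginPlay prunes invalid entries from the tracked AIActor array, then spawns enough to refill it.
; New AI appear at random X/Y offsets around the spawner, raised above it, and skip spawning if a collision-free spot cannot be found.
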(event Custom|CheckAI
  (for (_array_element _array_index) (Variables|Default|GetAIActor)
    (Utilities|IsValid _array_element
      (:Is%20Not%20Valid
        (Utilities|Array|RemoveIndex (Variables|Default|GetAIActor) _array_index))))
  (CallFunction|AIRespawn))

(event Custom|AIRespawn
  (bind _returnvalue (Transformation|GetActorLocation))
  (bind _aiactor (Variables|Default|GetAIActor))
  (bind _returnvalue_2 (Utilities|Array|Length _aiactor))
  (if (< _returnvalue_2 50)
    (for _index (range 1 (- 50 _returnvalue_2))
      (bind _returnvalue_3 (Game|SpawnActorfromClass "/Game/AI/AIBluePrints/BP_FriendAI.BP_FriendAI_C" (Math|Transform|MakeTransform (Math|Vector|MakeVector (Math|Random|RandomFloatinRange (- (.x _returnvalue) 1e+03) (+ (.x _returnvalue) 1e+03)) (Math|Random|RandomFloatinRange (- (.y _returnvalue) 1e+03) (+ (.y _returnvalue) 1e+03)) (+ (.z _returnvalue) 3e+02)) "0, 0, 0" "1.000000,1.000000,1.000000") "AdjustIfPossibleButDontSpawnIfColliding" "MultiplyWithRoot" 0 0))
      (Utilities|Array|Add (Variables|Default|GetAIActor) _returnvalue_3))))

(event EventBeginPlay
  (Utilities|Time|SetTimerbyEvent (delegate Custom|CheckAI) 1e+01 true))

(fn ConstructionScript)