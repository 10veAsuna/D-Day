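; Test Blueprint for an LCVP landing craft that drives itself forward and opens its door on a scripted timer.
; On BeginPlay, the Forward timeline immediately lerps the actor along world X from its starting position over a fixed distance.
; In parallel, after a delay, the Opendoor timeline lerps the Scene component's relative roll through a quarter turn to swing the door open.
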(event EventBeginPlay
  (bind _returnvalue (Transformation|GetActorLocation))
  (Variables|Default|SetReturn%20Value%20X (.x _returnvalue))
  (Utilities|FlowControl|Sequence
    (:then_0
      (Utilities|FlowControl|Delay 1e+01)
      (bind _新建轨道_0 (Timeline|opendoor PlayFromStart)
        (:Update
          (Transformation|SetRelativeRotation (Variables|Default|GetScene) (Math|Rotator|MakeRotator (Math|Float|Lerp 3.311 -86.689 _新建轨道_0) 0.0 0.0) false false))))
    (:then_1
      (bind _新建轨道_0_2 (Timeline|forward PlayFromStart)
        (:Update
          (Transformation|SetActorLocation (Math|Vector|MakeVector (Math|Float|Lerp (Variables|Default|GetReturn%20Value%20X) (+ (Variables|Default|GetReturn%20Value%20X) 5e+03) _新建轨道_0_2) (.y _returnvalue) (.z _returnvalue)) false false))))))

(fn ConstructionScript)