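; Enemy spawner actor that keeps up to 50 BP_EAI enemies around itself.
; A looping 10-second timer prunes invalid entries from AIActor, then spawns replacements at random XY offsets above the spawner.
; Box1 plays audio while a player-tagged actor overlaps it.
; Leaving Box removes the BP_Soldier's spawner-destruction UI and resets its DestoryBar progress.
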(event OnComponentBeginOverlap(Box1)
  (params (OverlappedComponent :type Primitive%20Component%20Object%20Reference) (OtherActor :type Actor%20Object%20Reference) (OtherComp :type Primitive%20Component%20Object%20Reference) (OtherBodyIndex :type Integer) (bFromSweep :type Boolean) (SweepResult :type Hit%20Result%20Structure%20%28by%20ref%29))
  (if (Actor|ActorHasTag OtherActor "player")
    (Audio|Components|Audio|Play (Variables|Default|GetAudio1) 0.0)))

(event OnComponentEndOverlap(Box1)
  (params (OverlappedComponent :type Primitive%20Component%20Object%20Reference) (OtherActor :type Actor%20Object%20Reference) (OtherComp :type Primitive%20Component%20Object%20Reference) (OtherBodyIndex :type Integer))
  (if (Actor|ActorHasTag OtherActor "player")
    (Audio|Components|Audio|Stop (Variables|Default|GetAudio1))))

(event OnComponentEndOverlap(Box)
  (params (OverlappedComponent :type Primitive%20Component%20Object%20Reference) (OtherActor :type Actor%20Object%20Reference) (OtherComp :type Primitive%20Component%20Object%20Reference) (OtherBodyIndex :type Integer))
  (if (Actor|ActorHasTag OtherActor "player")
    (bind _returnvalue (Actor|GetActorOfClass "/Game/BluePrints/Character/BP_Soldier.BP_Soldier_C"))
    (Utilities|FlowControl|Sequence
      (:then_0
        (bind _destoryenemyspawnui (Variables|/Game/BluePrints/Character/BP_Soldier.BP_Soldier_C|GetDestoryEnemySpawnUI _returnvalue)
          (:then
            (Widget|RemovefromParent _destoryenemyspawnui))
          (:else)))
      (:then_1
        (Variables|/Game/BluePrints/Character/BP_Soldier.BP_Soldier_C|SetDestoryBar _returnvalue 0.0)))))

(event Custom|CheckAI
  (for (_array_element _array_index) (Variables|Default|GetAIActor)
    (Utilities|IsValid _array_element
      (:Is%20Not%20Valid
        (Utilities|Array|RemoveIndex (Variables|Default|GetAIActor) _array_index))))
  (CallFunction|AIRespawn))

(event Custom|AIRespawn
  (bind _returnvalue (Transformation|GetActorLocation))
  (bind _aiactor (Variables|Default|GetAIActor))
  (bind _returnvalue_2 (Utilities|Array|Length _aiactor))
  (if (< _returnvalue_2 50)
    (for _index (range 1 (- 50 _returnvalue_2))
      (bind _returnvalue_3 (Game|SpawnActorfromClass "/Game/AI/AIBluePrints/BP_EAI.BP_EAI_C" (Math|Transform|MakeTransform (Math|Vector|MakeVector (Math|Random|RandomFloatinRange (- (.x _returnvalue) 1e+03) (+ (.x _returnvalue) 1e+03)) (Math|Random|RandomFloatinRange (- (.y _returnvalue) 1e+03) (+ (.y _returnvalue) 1e+03)) (+ (.z _returnvalue) 3e+02)) "0, 0, 0" "1.000000,1.000000,1.000000") "AdjustIfPossibleButDontSpawnIfColliding" "MultiplyWithRoot" 0 0))
      (Utilities|Array|Add (Variables|Default|GetAIActor) _returnvalue_3))))

(event EventBeginPlay
  (Utilities|Time|SetTimerbyEvent (delegate Custom|CheckAI) 1e+01 true))

(fn ConstructionScript)