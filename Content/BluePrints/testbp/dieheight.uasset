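; Trigger-box Blueprint that acts as a timed death zone for BP_Soldier, apparently for drowning, judging by the Drow widget name.
; On overlap begin it shows the Drow warning widget and starts a three-second timer; leaving the box cancels both.
; If the timer fires, the die event swaps the warning for the Die widget, without changing the soldier itself.
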(event OnComponentBeginOverlap(Box)
  (params (OverlappedComponent :type Primitive%20Component%20Object%20Reference) (OtherActor :type Actor%20Object%20Reference) (OtherComp :type Primitive%20Component%20Object%20Reference) (OtherBodyIndex :type Integer) (bFromSweep :type Boolean) (SweepResult :type Hit%20Result%20Structure%20%28by%20ref%29))
  (Development|PrintString "in")
  (bind _asbp_soldier (Utilities|Casting|CastToBP_Soldier OtherActor))
  (bind _returnvalue (UserInterface|CreateWidget "/Game/BluePrints/testbp/drow.drow_C"))
  (Variables|Default|Setdrowui _returnvalue)
  (UserInterface|Viewport|AddtoViewport (Variables|Default|Getdrowui) 0)
  (bind _returnvalue_2 (Utilities|Time|SetTimerbyEvent (delegate Custom|die) 3.0)))

(event OnComponentEndOverlap(Box)
  (params (OverlappedComponent :type Primitive%20Component%20Object%20Reference) (OtherActor :type Actor%20Object%20Reference) (OtherComp :type Primitive%20Component%20Object%20Reference) (OtherBodyIndex :type Integer))
  (Development|PrintString "out")
  (bind _asbp_soldier (Utilities|Casting|CastToBP_Soldier OtherActor))
  (Utilities|Time|ClearandInvalidateTimerbyHandle (stale OnComponentBeginOverlap(Box) _returnvalue_2))
  (Widget|RemovefromParent (Variables|Default|Getdrowui)))

(event Custom|die
  (Utilities|Time|ClearandInvalidateTimerbyHandle (stale OnComponentBeginOverlap(Box) _returnvalue_2))
  (Widget|RemovefromParent (Variables|Default|Getdrowui))
  (bind _returnvalue (UserInterface|CreateWidget "/Game/BluePrints/testbp/die.die_C"))
  (Variables|Default|Setdieui _returnvalue)
  (UserInterface|Viewport|AddtoViewport (Variables|Default|Getdieui) 0))

(event EventBeginPlay)

(fn ConstructionScript)