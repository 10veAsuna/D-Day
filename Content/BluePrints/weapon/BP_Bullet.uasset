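; BP_Bullet is a weapon projectile that damages overlapped actors tagged "person" and leaves bullet holes on impact.
; Overlap applies random damage based on BP_Controller's equipped Thompson or Garand, then triggers UI red-cross feedback and a Niagara damage number.
; The number's position reuses the Hit event's sphere trace result.
; Hit sphere-traces at the impact point, spawns a temporary surface-aligned decal and destroys the bullet.
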(event Custom|AddBulletHole
  (params (Location :type Vector) (Rotation :type Rotator))
  (Rendering|Decal|SpawnDecalatLocation "/Game/BluePrints/weapon/BulletHole.BulletHole" "7.000000,7.000000,7.000000" Location Rotation 1e+01))

(event Collision|EventActorBeginOverlap
  (params (OtherActor :type Actor%20Object%20Reference))
  (bind _self self)
  (if (Actor|ActorHasTag OtherActor "person")
    (bind _returnvalue (Actor|GetActorOfClass "/Game/BluePrints/BP_Controller.BP_Controller_C"))
    (switch Utilities|FlowControl|Switch|SwitchonENUM_WeaponType (Variables|/Game/BluePrints/BP_Controller.BP_Controller_C|GetEquippedWeapon _returnvalue)
      (:NewEnumerator0
        (bind _returnvalue_2 (Game|Damage|ApplyDamage OtherActor (Math|Random|RandomFloatinRange 1e+01 3e+01) 0 _self)))
      (:NewEnumerator1
        (Game|Damage|ApplyDamage OtherActor (Math|Random|RandomFloatinRange 4e+01 6e+01) 0 _self)))
    (bind _foundwidgets (Class|WidgetBlueprintLibrary|GetAllWidgetswithInterface "/Game/API/API_UI.API_UI_C" false))
    (Class|APIUI|RedCross(Message) _foundwidgets)
    (bind _returnvalue_3 (Niagara|SpawnSystematLocation "/Game/BluePrints/weapon/NS_DamageValue.NS_DamageValue" (.Location (Collision|BreakHitResult (stale Collision|EventHit _outhit)))))
    (Class|NiagaraComponent|SetVariableInt _returnvalue_3 "Number" (Math|Float|Truncate _returnvalue_2))
    (Development|PrintString (Utilities|String|ToString(Integer) (Math|Float|Truncate _returnvalue_2)))))

(event Collision|EventHit
  (params (MyComp :type Primitive%20Component%20Object%20Reference) (Other :type Actor%20Object%20Reference) (OtherComp :type Primitive%20Component%20Object%20Reference) (bSelfMoved :type Boolean) (HitLocation :type Vector :default "0, 0, 0") (HitNormal :type Vector :default "0, 0, 0") (NormalImpulse :type Vector :default "0, 0, 0") (Hit :type Hit%20Result%20Structure%20%28by%20ref%29))
  (bind _outhit (Collision|SphereTraceByChannel HitLocation HitLocation 2.0 "TraceTypeQuery1" false 0 "ForDuration"))
  (CallFunction|AddBulletHole (.Location (Collision|BreakHitResult _outhit)) (Math|Conversions|RotationFromXVector (.Normal (Collision|BreakHitResult _outhit))))
  (Actor|DestroyActor))

(fn ConstructionScript)