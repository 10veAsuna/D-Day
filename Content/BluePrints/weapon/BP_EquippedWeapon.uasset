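; BP_EquippedWeapon is the equipped gun actor, taking its starting bullet count from a weapon data asset.
; Fire plays a dry-fire sound when empty, otherwise triggers recoil, muzzle flash and sound, then decrements ammo.
; A debug-drawn camera trace aims a BP_Bullet spawned at the muzzle socket and directly applies random damage to "person"-tagged actors.
; A timeline drives pitch recoil, then reverses at reduced strength; yaw recoil is unconnected.
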(event Custom|Recoil
  (bind (_direction _recoil) (Timeline|RecoilRelease PlayFromStart)
    (:Update
      (switch Utilities|FlowControl|Switch|SwitchonETimelineDirection _direction
        (:Forward
          (Pawn|Input|AddControllerPitchInput (Game|Player|GetPlayerPawn 0) (Math|Float|Lerp 0.0 (Variables|Default|GetRecoilP) _recoil)))
        (:Backward
          (Pawn|Input|AddControllerPitchInput (Game|Player|GetPlayerPawn 0) (* (Math|Float|Lerp 0.0 (Variables|Default|GetRecoilP) _recoil) -0.1)))))
    (:Finished
      (CallFunction|Back))))

(event Custom|Back
  (bind (_direction _recoil) (Timeline|RecoilRelease Reverse)
    (:Update
      (switch Utilities|FlowControl|Switch|SwitchonETimelineDirection _direction
        (:Forward
          (Pawn|Input|AddControllerPitchInput (Game|Player|GetPlayerPawn 0) (Math|Float|Lerp 0.0 (Variables|Default|GetRecoilP) _recoil)))
        (:Backward
          (Pawn|Input|AddControllerPitchInput (Game|Player|GetPlayerPawn 0) (* (Math|Float|Lerp 0.0 (Variables|Default|GetRecoilP) _recoil) -0.1)))))
    (:Finished
      (CallFunction|Back))))

(event EventBeginPlay
  (Variables|Default|SetBulletNumber (.weaponbulletsnumber (Variables|/Game/BluePrints/weapon/BP_Weapon.BP_Weapon_C|GetWeaponAttri (Variables|Default|GetWeaponDataAsset)))))

(event EventFire
  (bind _returnvalue (Game|GetPlayerCameraManager 0))
  (bind _skeletalmesh (Variables|Default|GetSkeletalMesh))
  (bind _skeletalmesh_2 (Variables|Default|GetSkeletalMesh))
  (bind _returnvalue_2 (Transformation|GetSocketTransform _skeletalmesh "Fire" "RTS_World"))
  (bind _returnvalue_3 (Camera|GetCameraLocation _returnvalue))
  (bind _returnvalue_4 (Transformation|GetSocketTransform _skeletalmesh_2 "Fire" "RTS_World"))
  (if (== (Variables|Default|GetBulletNumber) 0)
    (Audio|PlaySoundatLocation "/Game/Anim/Audio/Sounds/Weapons/Rifle/A_Weapons_Rifle_DryFire_01.A_Weapons_Rifle_DryFire_01" (.location _returnvalue_4) "0, 0, 0" 1.0 1.0 0.0 0 0 0 0)
    (else
      (CallFunction|Recoil)
      (bind _returnvalue_5 (Niagara|SpawnSystematLocation "/Game/BluePrints/weapon/FXS_MuzzleFlash.FXS_MuzzleFlash" (.location _returnvalue_4) (.rotation _returnvalue_4)))
      (Audio|PlaySoundatLocation (Variables|Default|GetSound) (.location _returnvalue_4) "0, 0, 0" 1.0 1.0 0.0 0 0 0 0)
      (Transformation|AttachComponentToComponent _returnvalue_5 (Variables|Default|GetSkeletalMesh) "Fire" "KeepRelative" "KeepRelative" "KeepRelative" true)
      (bind (_outhit _returnvalue_6) (Collision|LineTraceByChannel _returnvalue_3 (+ _returnvalue_3 (* (Math|Vector|GetForwardVector (Camera|GetCameraRotation _returnvalue)) 20000)) "TraceTypeQuery1" false 0 "ForDuration" false))
      (Game|SpawnActorfromClass "/Game/BluePrints/weapon/BP_Bullet.BP_Bullet_C" (Math|Transform|MakeTransform (.location _returnvalue_2) (Math|Rotator|FindLookatRotation (.location _returnvalue_2) (select _returnvalue_6 (.Location (Collision|BreakHitResult _outhit)) (.TraceEnd (Collision|BreakHitResult _outhit)))) "1.000000,1.000000,1.000000") "AlwaysSpawn" "MultiplyWithRoot" 0 0)
      (Math|Integer|DecrementInt (Variables|Default|GetBulletNumber)
        (:%20%20
          (Utilities|IsValid (.HitActor (Collision|BreakHitResult _outhit))
            (:Is%20Valid
              (if (Actor|ActorHasTag (.HitActor (Collision|BreakHitResult _outhit)) "person")
                (bind _returnvalue_7 (Game|Damage|ApplyDamage (.HitActor (Collision|BreakHitResult _outhit)) (Math|Random|RandomFloatinRange 5.0 2e+01) 0 0))
                (Development|PrintString (Utilities|String|ToString(Float) _returnvalue_7) true true "(R=0.006380,G=1.000000,B=0.167915,A=1.000000)")))))))))

(fn ConstructionScript)

(fn GetEquippedWeaponDataAsset
  (return (Variables|Default|GetWeaponDataAsset)))