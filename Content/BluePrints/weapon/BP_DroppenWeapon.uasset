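; BP_DroppenWeapon is a dropped weapon in the world, defined by a weapon data asset.
; The construction script sets its static mesh from that asset, and BeginPlay enables physics simulation on the mesh.
; Highlight events set and clear an Interact overlay material on the mesh, and a getter exposes the data asset to other objects.
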(event EventBeginPlay
  (Physics|SetSimulatePhysics (Variables|Default|GetStaticMesh) true))

(event EventTurnOffHighlighting
  (Rendering|Material|SetOverlayMaterial (Variables|Default|GetStaticMesh) 0 :!class /Script/Engine.MeshComponent))

(event EventTurnonHighlighting
  (Rendering|Material|SetOverlayMaterial (Variables|Default|GetStaticMesh) "/Game/BluePrints/weapon/Interact.Interact" :!class /Script/Engine.MeshComponent))

(fn ConstructionScript
  (Components|StaticMesh|SetStaticMesh (Variables|Default|GetStaticMesh) (Variables|/Game/BluePrints/weapon/BP_Weapon.BP_Weapon_C|GetStatic (Variables|Default|GetWeaponDataAsset))))

(fn GetWeaponDataAsset
  (return (Variables|Default|GetWeaponDataAsset)))