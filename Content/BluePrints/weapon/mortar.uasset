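; Mortar weapon Blueprint that lets player input aim it horizontally and vertically through two scene components.
; The turn action adds scaled input to the world yaw of Scene.
; Separate up and down actions adjust the pitch of Scene1, each checking one limit of a narrow range before stepping.
; Pitch updates read world rotation but write it back as relative rotation.
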(event Input|EnhancedActionEvents|EnhancedInputActionIAmortar_turn
  (params (ActionValue :type Float%20%28double-precision%29) (ElapsedSeconds :type Float%20%28double-precision%29) (TriggeredSeconds :type Float%20%28double-precision%29) (InputAction :type Input%20Action%20Object%20Reference :default "/Game/Input/mortar/IAmortar_turn.IAmortar_turn"))
  (bind _scene (Variables|Default|GetScene))
  (bind _returnvalue (Transformation|GetWorldRotation _scene))
  ;[0.15 0.15 0.15 0.5] 左右
  (Transformation|SetWorldRotation _scene (Math|Rotator|MakeRotator (.roll _returnvalue) (.pitch _returnvalue) (+ (* ActionValue 0.5) (.yaw _returnvalue))) false false))

(event Input|EnhancedActionEvents|EnhancedInputActionIAmortar_up
  (params (ActionValue :type Float%20%28double-precision%29) (ElapsedSeconds :type Float%20%28double-precision%29) (TriggeredSeconds :type Float%20%28double-precision%29) (InputAction :type Input%20Action%20Object%20Reference :default "/Game/Input/mortar/IAmortar_up.IAmortar_up"))
  (bind _scene1 (Variables|Default|GetScene1))
  (bind _returnvalue (Transformation|GetWorldRotation _scene1))
  ;[0.15 0.15 0.15 0.5] 上下
  (if (<= (.pitch (Transformation|GetWorldRotation (Variables|Default|GetScene1))) 1e+01)
    (Transformation|SetRelativeRotation _scene1 (Math|Rotator|MakeRotator (.roll _returnvalue) (+ (* ActionValue 0.5) (.pitch _returnvalue)) (.yaw _returnvalue)) false false)))

(event Input|EnhancedActionEvents|EnhancedInputActionIAmortar_down
  (params (ActionValue :type Float%20%28double-precision%29) (ElapsedSeconds :type Float%20%28double-precision%29) (TriggeredSeconds :type Float%20%28double-precision%29) (InputAction :type Input%20Action%20Object%20Reference :default "/Game/Input/mortar/IAmortar_down.IAmortar_down"))
  (bind _scene1 (Variables|Default|GetScene1))
  (bind _returnvalue (Transformation|GetWorldRotation _scene1))
  ;[0.15 0.15 0.15 0.5] 上下
  (if (>= (.pitch (Transformation|GetWorldRotation (Variables|Default|GetScene1))) -1e+01)
    (Transformation|SetRelativeRotation _scene1 (Math|Rotator|MakeRotator (.roll _returnvalue) (+ (* ActionValue 0.5) (.pitch _returnvalue)) (.yaw _returnvalue)) false false)))

(fn ConstructionScript)