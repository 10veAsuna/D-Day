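; First-person player character Blueprint (玩家_BP) handling Enhanced Input movement, sprint, crouch, weapon pickup, switching, firing, reloading and ADS.
; An action-state enum gates inputs, while timelines drive crouch height, weapon-swap arm lowering and aim FOV.
; A per-tick camera trace highlights pickups, spawned from data assets into pistol/rifle slots and socketed to back or hand.
; It feeds weapon/aim state to 玩家_ABP, ammo to the HUD, and provides surface-based footstep sounds.
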(event EventBeginPlay
  (bind _returnvalue (Game|GetPlayerController 0))
  (bind _returnvalue_2 (Game|GetPlayerCameraManager 0))
  (bind _returnvalue_3 (PlayerController|LocalPlayerSubsystems|GetEnhancedInputLocalPlayerSubsystem _returnvalue))
  (Utilities|IsValid _returnvalue_3
    (:Is%20Valid
      (Input|AddMappingContext _returnvalue_3 "/Game/输入/FPS增强输入.FPS增强输入" 0 "(bIgnoreAllPressedKeysUntilRelease=True,bForceImmediately=False,bNotifyUserSettings=False)")
      (Variables|/Script/Engine.PlayerCameraManager|SetViewPitchMin _returnvalue_2 -75.0)
      (Variables|/Script/Engine.PlayerCameraManager|SetViewPitchMax _returnvalue_2 75.0)
      (bind _returnvalue_4 (UserInterface|CreateWidget "/Game/HUD/HUD.HUD_C"))
      (bind _output_get (Variables|Default|SetHUD _returnvalue_4))
      (UserInterface|Viewport|AddtoViewport _output_get 0)
      (bind _as玩家_abp (Utilities|Casting|CastTo玩家_ABP (Components|SkeletalMesh|GetAnimInstance (Variables|Default|GetFPS_SkeletalMesh))))
      (Variables|Default|SetAs玩家%20ABP _as玩家_abp))))

(event Input|EnhancedActionEvents|EnhancedInputActionIA_移动
  (params (ActionValue :type Vector%202D%20Structure) (ElapsedSeconds :type Float%20%28double-precision%29) (TriggeredSeconds :type Float%20%28double-precision%29) (InputAction :type Input%20Action%20Object%20Reference :default "/Game/输入/IA_移动.IA_移动"))
  (bind (_x _y) (Math|Vector2D|BreakVector2D ActionValue))
  ;[1 1 1] 移动
  (Pawn|Input|AddMovementInput (Transformation|GetActorRightVector) _x false)
  (Pawn|Input|AddMovementInput (Transformation|GetActorForwardVector) _y false))

(event Input|EnhancedActionEvents|EnhancedInputActionIA_查看
  (params (ActionValue :type Vector%202D%20Structure) (ElapsedSeconds :type Float%20%28double-precision%29) (TriggeredSeconds :type Float%20%28double-precision%29) (InputAction :type Input%20Action%20Object%20Reference :default "/Game/输入/IA_查看.IA_查看"))
  (bind (_x _y) (Math|Vector2D|BreakVector2D ActionValue))
  ;[1 1 1] 查看
  (Pawn|Input|AddControllerYawInput _x)
  (Pawn|Input|AddControllerPitchInput _y))

(event Input|EnhancedActionEvents|EnhancedInputActionIA_跳跃
  (params (ActionValue :type Boolean) (ElapsedSeconds :type Float%20%28double-precision%29) (TriggeredSeconds :type Float%20%28double-precision%29) (InputAction :type Input%20Action%20Object%20Reference :default "/Game/输入/IA_跳跃.IA_跳跃"))
  ;[1 1 1] 跳和跑
  (:Started
    (switch Utilities|FlowControl|Switch|SwitchonE_玩家动作 (Variables|Default|Get玩家动作)
      (:NewEnumerator0
        _)
      (:NewEnumerator1
        _))
    (Character|Jump))
  (:Completed
    (Character|StopJumping)))

(event Input|EnhancedActionEvents|EnhancedInputActionIA_加速跑
  (params (ActionValue :type Boolean) (ElapsedSeconds :type Float%20%28double-precision%29) (TriggeredSeconds :type Float%20%28double-precision%29) (InputAction :type Input%20Action%20Object%20Reference :default "/Game/输入/IA_加速跑.IA_加速跑"))
  (bind _玩家动作 (Variables|Default|Get玩家动作))
  ;[1 1 1] 跳和跑
  (:Started
    (switch Utilities|FlowControl|Switch|SwitchonE_玩家动作 _玩家动作
      (:NewEnumerator0
        (Utilities|改变玩家移动速度 "NewEnumerator1"))))
  (:Completed
    (switch Utilities|FlowControl|Switch|SwitchonE_玩家动作 _玩家动作
      (:NewEnumerator1
        (Utilities|改变玩家移动速度 "NewEnumerator0")))))

(event Input|EnhancedActionEvents|EnhancedInputActionIA_蹲伏
  (params (ActionValue :type Boolean) (ElapsedSeconds :type Float%20%28double-precision%29) (TriggeredSeconds :type Float%20%28double-precision%29) (InputAction :type Input%20Action%20Object%20Reference :default "/Game/输入/IA_蹲伏.IA_蹲伏"))
  ;[1 1 1] 蹲伏
  (:Started
    (switch Utilities|FlowControl|Switch|SwitchonE_玩家动作 (Variables|Default|Get玩家动作)
      (:NewEnumerator0
        (Utilities|改变玩家移动速度 "NewEnumerator3" :!label _label)
        (bind _新建轨道_0 (Timeline|胶囊体蹲伏设置 Play)
          (:Update
            (Components|Capsule|SetCapsuleHalfHeight (Variables|Collision|GetCapsuleComponent) (Math|Float|Lerp 88.0 6e+01 _新建轨道_0) true))))
      (:NewEnumerator1
        (goto _label))
      (:NewEnumerator3
        (bind _是否检测到 (Utilities|蹲伏障碍物检测))
        (if (not _是否检测到)
          (Utilities|改变玩家移动速度 "NewEnumerator0")
          (Timeline|胶囊体蹲伏设置 Reverse))))))

(event EventTick
  (params (DeltaSeconds :type Float%20%28single-precision%29))
  (Utilities|交互物品视线检测))

(event Custom|放下手
  (params (目标 :type Actor%20Object%20Reference))
  ;[1 1 1] 抬手放手
  (bind (_direction _新建轨道_0) (Timeline|放手 PlayFromStart)
    (:Update
      (Transformation|SetRelativeLocation (Variables|Default|GetFPS_SkeletalMesh) (Math|Vector|MakeVector 0.0 0.0 (Math|Float|Lerp -165.0 -2.1e+02 _新建轨道_0)) false false))
    (:Finished
      (switch Utilities|FlowControl|Switch|SwitchonETimelineDirection _direction
        (:Forward
          (Utilities|把所有武器放回后背
            (:结束
              (bind _returnvalue (Utilities|武器放到手里 目标))
              (if _returnvalue
                (bind _资产 (Class|装备的武器接口|获取装备的武器数据资产(Message) 目标))
                (bind _output_get (Variables|Default|Set装备的武器 (Variables|/Game/数据资产/武器_数据资产.武器_数据资产_C|Get武器名 _资产)))
                (Variables|/Game/玩家蓝图/玩家_ABP.玩家_ABP_C|Set装备的武器 (Variables|Default|GetAs玩家%20ABP) _output_get)
                (Utilities|FlowControl|Delay 0.2)
                (CallFunction|抬起手)))))
        (:Backward
          (CallFunction|更新子弹显示UI))))))

(event Custom|抬起手
  ;[1 1 1] 抬手放手
  (bind (_direction _新建轨道_0) (Timeline|放手 Reverse)
    (:Update
      (Transformation|SetRelativeLocation (Variables|Default|GetFPS_SkeletalMesh) (Math|Vector|MakeVector 0.0 0.0 (Math|Float|Lerp -165.0 -2.1e+02 _新建轨道_0)) false false))
    (:Finished
      (switch Utilities|FlowControl|Switch|SwitchonETimelineDirection _direction
        (:Forward
          (Utilities|把所有武器放回后背
            (:结束
              (bind _returnvalue (Utilities|武器放到手里 (stale Custom|放下手 目标)))
              (if _returnvalue
                (bind _资产 (Class|装备的武器接口|获取装备的武器数据资产(Message) (stale Custom|放下手 目标)))
                (bind _output_get (Variables|Default|Set装备的武器 (Variables|/Game/数据资产/武器_数据资产.武器_数据资产_C|Get武器名 _资产)))
                (Variables|/Game/玩家蓝图/玩家_ABP.玩家_ABP_C|Set装备的武器 (Variables|Default|GetAs玩家%20ABP) _output_get)
                (Utilities|FlowControl|Delay 0.2)
                (CallFunction|抬起手)))))
        (:Backward
          (CallFunction|更新子弹显示UI))))))

(event Custom|更新子弹显示UI
  (bind _hud (Variables|Default|GetHUD))
  ;[1 1 1] 抬手放手
  (Class|HUD接口|显示子弹数(Message) _hud)
  (Class|HUD接口|UI更新子弹数(Message) _hud (Utilities|Select :Index (Variables|Default|Get手持武器状态) :NewEnumerator0 0 :NewEnumerator1 (Variables|/Game/武器蓝图/装备的武器_BP.装备的武器_BP_C|Get弹匣子弹数 (Variables|Default|Get装备的武器_手枪)) :NewEnumerator4 (Variables|/Game/武器蓝图/装备的武器_BP.装备的武器_BP_C|Get弹匣子弹数 (Variables|Default|Get装备的武器_步枪))) (Utilities|Select :Index (Variables|Default|Get手持武器状态) :NewEnumerator0 0 :NewEnumerator1 (Variables|Default|Get玩家携带手枪子弹) :NewEnumerator4 (Variables|Default|Get玩家携带步枪子弹))))

(event Custom|瞄准切换
  (params (玩家瞄准 :type Boolean))
  (bind _output_get (Variables|Default|Set玩家瞄准 玩家瞄准))
  (Variables|/Game/玩家蓝图/玩家_ABP.玩家_ABP_C|Set玩家瞄准 (Variables|Default|GetAs玩家%20ABP) _output_get))

(event Input|EnhancedActionEvents|EnhancedInputActionIA_拾取
  (params (ActionValue :type Boolean) (ElapsedSeconds :type Float%20%28double-precision%29) (TriggeredSeconds :type Float%20%28double-precision%29) (InputAction :type Input%20Action%20Object%20Reference :default "/Game/输入/IA_拾取.IA_拾取"))
  ;[1 1 1] 拾取
  (:Started
    (Variables|Default|Get交互Actor
      (:then
        (bind _资产 (Class|掉落的武器接口|获取数据资产(Message) (Variables|Default|Get交互Actor)))
        (bind _returnvalue (Game|SpawnActorfromClass (Variables|/Game/数据资产/武器_数据资产.武器_数据资产_C|Get武器类 _资产) (Math|Transform|MakeTransform "0, 0, 0" "0, 0, 0" "1.000000,1.000000,1.000000") "AlwaysSpawn" "MultiplyWithRoot" 0 _资产 0))
        (switch Utilities|FlowControl|Switch|SwitchonE_武器分类 (Variables|/Game/数据资产/武器_数据资产.武器_数据资产_C|Get武器分类 _资产)
          (:NewEnumerator1
            (bind _装备的武器_手枪 (Variables|Default|Get装备的武器_手枪)
              (:then
                (switch Utilities|FlowControl|Switch|SwitchonE_武器分类 (Variables|Default|Get手持武器状态)
                  (:NewEnumerator0
                    (Utilities|拾取新武器丢弃旧武器 (Variables|/Game/武器蓝图/装备的武器_BP.装备的武器_BP_C|Get武器数据资产 _装备的武器_手枪) :!label _label)
                    (bind _output_get (Variables|Default|Set装备的武器_手枪 _returnvalue :!label _label_2))
                    (bind _returnvalue_2 (Utilities|武器放到后背 _output_get))
                    (if _returnvalue_2
                      (Actor|DestroyActor (Variables|Default|Get交互Actor) :!label _label_3)
                      (Variables|Default|Set交互Actor 0)))
                  (:NewEnumerator1
                    (Utilities|拾取新武器丢弃旧武器 (Variables|/Game/武器蓝图/装备的武器_BP.装备的武器_BP_C|Get武器数据资产 _装备的武器_手枪))
                    (bind _output_get_2 (Variables|Default|Set装备的武器_手枪 _returnvalue))
                    (CallFunction|放下手 _output_get_2)
                    (goto _label_3))
                  (:NewEnumerator4
                    (goto _label))))
              (:else
                (goto _label_2))))
          (:NewEnumerator4
            (bind _装备的武器_步枪 (Variables|Default|Get装备的武器_步枪)
              (:then
                (switch Utilities|FlowControl|Switch|SwitchonE_武器分类 (Variables|Default|Get手持武器状态)
                  (:NewEnumerator0
                    _)
                  (:NewEnumerator1
                    _)
                  (:NewEnumerator4
                    (Utilities|拾取新武器丢弃旧武器 (Variables|/Game/武器蓝图/装备的武器_BP.装备的武器_BP_C|Get武器数据资产 _装备的武器_步枪))
                    (bind _output_get_3 (Variables|Default|Set装备的武器_步枪 _returnvalue))
                    (CallFunction|放下手 _output_get_3)
                    (goto _label_3)))
                (Utilities|拾取新武器丢弃旧武器 (Variables|/Game/武器蓝图/装备的武器_BP.装备的武器_BP_C|Get武器数据资产 _装备的武器_步枪)))
              (:else
                _))
            (bind _output_get_4 (Variables|Default|Set装备的武器_步枪 _returnvalue))
            (bind _returnvalue_3 (Utilities|武器放到后背 _output_get_4))
            (if _returnvalue_3
              (goto _label_3)))))
      (:else))))

(event Input|EnhancedActionEvents|EnhancedInputActionIA_1
  (params (ActionValue :type Boolean) (ElapsedSeconds :type Float%20%28double-precision%29) (TriggeredSeconds :type Float%20%28double-precision%29) (InputAction :type Input%20Action%20Object%20Reference :default "/Game/输入/IA_1.IA_1"))
  ;[1 1 1] 装备
  (:Started
    (bind _装备的武器_手枪 (Variables|Default|Get装备的武器_手枪)
      (:then
        (CallFunction|放下手 _装备的武器_手枪)
        (Variables|Default|Set手持武器状态 "NewEnumerator1"))
      (:else))))

(event Input|EnhancedActionEvents|EnhancedInputActionIA_2
  (params (ActionValue :type Boolean) (ElapsedSeconds :type Float%20%28double-precision%29) (TriggeredSeconds :type Float%20%28double-precision%29) (InputAction :type Input%20Action%20Object%20Reference :default "/Game/输入/IA_2.IA_2"))
  ;[1 1 1] 装备
  (:Started
    (bind _装备的武器_步枪 (Variables|Default|Get装备的武器_步枪)
      (:then
        (CallFunction|放下手 _装备的武器_步枪)
        (Variables|Default|Set手持武器状态 "NewEnumerator4"))
      (:else))))

(event Input|EnhancedActionEvents|EnhancedInputActionIA_开火
  (params (ActionValue :type Boolean) (ElapsedSeconds :type Float%20%28double-precision%29) (TriggeredSeconds :type Float%20%28double-precision%29) (InputAction :type Input%20Action%20Object%20Reference :default "/Game/输入/IA_开火.IA_开火"))
  (bind _装备的武器_手枪 (Variables|Default|Get装备的武器_手枪))
  (bind _装备的武器_步枪 (Variables|Default|Get装备的武器_步枪))
  ;[1 1 1] 开火
  (switch Utilities|FlowControl|Switch|SwitchonE_玩家动作 (Variables|Default|Get玩家动作)
    (:NewEnumerator0
      _)
    (:NewEnumerator3
      _))
  (switch Utilities|FlowControl|Switch|SwitchonE_武器分类 (Variables|Default|Get手持武器状态)
    (:NewEnumerator1
      (Variables|Default|Set玩家动作 "NewEnumerator4")
      (Class|装备的武器接口|开火(Message) _装备的武器_手枪)
      (Variables|Default|Set手部射击动画 (Variables|/Game/武器蓝图/装备的武器_BP.装备的武器_BP_C|Get武器手部射击动画 _装备的武器_手枪))
      (Variables|Default|Set手部射击动画_ADS (Variables|/Game/武器蓝图/装备的武器_BP.装备的武器_BP_C|Get武器手部射击动画_ADS _装备的武器_手枪))
      (Variables|Default|Set武器射击速率 (Variables|/Game/数据资产/武器_数据资产.武器_数据资产_C|Get射速 (Variables|/Game/武器蓝图/装备的武器_BP.装备的武器_BP_C|Get武器数据资产 _装备的武器_手枪))))
    (:NewEnumerator4
      (Variables|Default|Set玩家动作 "NewEnumerator4")
      (Class|装备的武器接口|开火(Message) _装备的武器_步枪)
      (Variables|Default|Set手部射击动画 (Variables|/Game/武器蓝图/装备的武器_BP.装备的武器_BP_C|Get武器手部射击动画 _装备的武器_步枪))
      (Variables|Default|Set手部射击动画_ADS (Variables|/Game/武器蓝图/装备的武器_BP.装备的武器_BP_C|Get武器手部射击动画_ADS _装备的武器_步枪))
      (Variables|Default|Set武器射击速率 (Variables|/Game/数据资产/武器_数据资产.武器_数据资产_C|Get射速 (Variables|/Game/武器蓝图/装备的武器_BP.装备的武器_BP_C|Get武器数据资产 _装备的武器_步枪)))))
  (CallFunction|更新子弹显示UI)
  (Animation|Montage|PlayMontage (Variables|Default|GetFPS_SkeletalMesh) (select (Variables|Default|Get玩家瞄准) (Variables|Default|Get手部射击动画_ADS) (Variables|Default|Get手部射击动画)) (Variables|Default|Get武器射击速率)
    (:OnCompleted
      (Utilities|恢复默认动作))))

(event Input|EnhancedActionEvents|EnhancedInputActionIA_上弹
  (params (ActionValue :type Boolean) (ElapsedSeconds :type Float%20%28double-precision%29) (TriggeredSeconds :type Float%20%28double-precision%29) (InputAction :type Input%20Action%20Object%20Reference :default "/Game/输入/IA_上弹.IA_上弹"))
  ;[1 1 1] 上弹
  (:Started
    (switch Utilities|FlowControl|Switch|SwitchonE_玩家动作 (Variables|Default|Get玩家动作)
      (:NewEnumerator0
        _)
      (:NewEnumerator3
        _))
    (Utilities|判断是否可以上弹
      (:是
        (Variables|Default|Set玩家动作 "NewEnumerator5")
        (switch Utilities|FlowControl|Switch|SwitchonE_武器 (Variables|Default|Get装备的武器)
          (:NewEnumerator1
            (Variables|Default|Set上弹动画 "/Game/IBFPSStarterPack/Animations/Arms/ANIM_ArK-47_Reload_Montage.ANIM_ArK-47_Reload_Montage"))
          (:NewEnumerator2
            (Variables|Default|Set上弹动画 "/Game/IBFPSStarterPack/Animations/Arms/ANIM_G18_Reload_Montage.ANIM_G18_Reload_Montage"))
          (:NewEnumerator4
            (Variables|Default|Set上弹动画 "/Game/IBFPSStarterPack/Animations/Arms/ANIM_XM8_Reload_Montage.ANIM_XM8_Reload_Montage"))
          (:NewEnumerator5
            (Variables|Default|Set上弹动画 "/Game/IBFPSStarterPack/Animations/Arms/ANIM_DesertEagle_Reload_Montage.ANIM_DesertEagle_Reload_Montage")))
        (Animation|Montage|PlayMontage (Variables|Default|GetFPS_SkeletalMesh) (Variables|Default|Get上弹动画)
          (:then
            (switch Utilities|FlowControl|Switch|SwitchonE_武器分类 (Variables|Default|Get手持武器状态)
              (:NewEnumerator1
                (Class|装备的武器接口|武器上弹(Message) (Variables|Default|Get装备的武器_手枪)))
              (:NewEnumerator4
                (Class|装备的武器接口|武器上弹(Message) (Variables|Default|Get装备的武器_步枪)))))
          (:OnCompleted
            (CallFunction|更新子弹显示UI)
            (Utilities|恢复默认动作)))))))

(event Input|EnhancedActionEvents|EnhancedInputActionIA_瞄准
  (params (ActionValue :type Boolean) (ElapsedSeconds :type Float%20%28double-precision%29) (TriggeredSeconds :type Float%20%28double-precision%29) (InputAction :type Input%20Action%20Object%20Reference :default "/Game/输入/IA_瞄准.IA_瞄准"))
  (:Started
    (switch Utilities|FlowControl|Switch|SwitchonE_武器分类 (Variables|Default|Get手持武器状态)
      (:NewEnumerator1
        _)
      (:NewEnumerator4
        _))
    (switch Utilities|FlowControl|Switch|SwitchonE_玩家动作 (Variables|Default|Get玩家动作)
      (:NewEnumerator0
        _)
      (:NewEnumerator3
        _)
      (:NewEnumerator4
        _))
    (CallFunction|瞄准切换 true)
    (bind _新建轨道_0 (Timeline|改变瞄准视角 Play)
      (:Update
        (Variables|/Script/Engine.CameraComponent|SetFieldOfView (Variables|Default|GetCamera) (Math|Float|Lerp 9e+01 7e+01 _新建轨道_0))
        (Transformation|SetRelativeLocation (Variables|Default|GetFPS_SkeletalMesh) (Math|Vector|MakeVector 0.0 0.0 (Math|Float|Lerp -165.0 (Utilities|Select :Index (Variables|Default|Get装备的武器) :NewEnumerator0 -165.0 :NewEnumerator1 -167.0 :NewEnumerator2 -165.0 :NewEnumerator4 -164.0 :NewEnumerator5 -165.0) _新建轨道_0)) false false))))
  (:Completed
    (switch Utilities|FlowControl|Switch|SwitchonE_武器分类 (Variables|Default|Get手持武器状态)
      (:NewEnumerator1
        _)
      (:NewEnumerator4
        _))
    (CallFunction|瞄准切换 false)
    (Timeline|改变瞄准视角 Reverse)))

(fn ConstructionScript)

(fn 脚步材质检测
  (bind _capsulecomponent (Variables|Collision|GetCapsuleComponent))
  (bind _returnvalue (Components|Capsule|GetScaledCapsuleHalfHeight _capsulecomponent))
  (bind _returnvalue_2 (Transformation|GetWorldLocation _capsulecomponent))
  (bind _returnvalue_3 (- _returnvalue_2 (Math|Vector|MakeVector 0.0 0.0 _returnvalue)))
  (bind (_outhit _returnvalue_4) (Collision|LineTraceByChannel _returnvalue_3 (- _returnvalue_3 "0.000000,0.000000,10.000000") "TraceTypeQuery3" false 0 "None"))
  (if _returnvalue_4
    (switch Utilities|FlowControl|Switch|SwitchonEPhysicalSurface (Collision|GetSurfaceType _outhit)
      (:SurfaceType_Default
        (LocalVariables|Set脚步音效 "/Game/音效/脚步音效_泥土.脚步音效_泥土"))
      (:SurfaceType1
        (LocalVariables|Set脚步音效 "/Game/音效/脚步音效_金属.脚步音效_金属"))
      (:SurfaceType2
        (LocalVariables|Set脚步音效 "/Game/音效/脚步音效_混凝土.脚步音效_混凝土"))
      (:SurfaceType3
        (LocalVariables|Set脚步音效 "/Game/音效/脚步音效_水.脚步音效_水"))
      (:SurfaceType4
        (LocalVariables|Set脚步音效 "/Game/音效/脚步音效_泥土.脚步音效_泥土"))
      (:SurfaceType5
        (LocalVariables|Set脚步音效 "/Game/音效/脚步音效_木头.脚步音效_木头"))
      (:SurfaceType6
        (LocalVariables|Set脚步音效 "/Game/音效/脚步音效_植物.脚步音效_植物")))
    (Audio|PlaySoundatLocation (LocalVariables|Get脚步音效) (.Location (Collision|BreakHitResult _outhit)) "0, 0, 0" 0.2 1.0 0.0 0 0 0 0)))