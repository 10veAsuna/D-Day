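; Dropped weapon pickup Blueprint that represents a weapon lying in the world as a physics-simulated static mesh.
; The construction script takes the mesh from the weapon data asset (武器数据资产), and BeginPlay turns on physics simulation.
; Highlight events 高亮显示 and 关闭高亮 set and clear an interaction overlay material on the mesh.
; 获取数据资产 returns the data asset to callers.
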(event EventBeginPlay
  (Physics|SetSimulatePhysics (Variables|Default|GetStaticMesh) true))

(event Event关闭高亮
  (Rendering|Material|SetOverlayMaterial (Variables|Default|GetStaticMesh) 0 :!class /Script/Engine.MeshComponent))

(event Event高亮显示
  (Rendering|Material|SetOverlayMaterial (Variables|Default|GetStaticMesh) "/Game/材质/交互材质.交互材质" :!class /Script/Engine.MeshComponent))

(fn ConstructionScript
  (Components|StaticMesh|SetStaticMesh (Variables|Default|GetStaticMesh) (Variables|/Game/数据资产/武器_数据资产.武器_数据资产_C|Get静态 (Variables|Default|Get武器数据资产))))

(fn 获取数据资产
  (return (Variables|Default|Get武器数据资产)))