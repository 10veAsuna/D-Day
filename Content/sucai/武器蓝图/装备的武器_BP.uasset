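; Equipped weapon actor that handles firing, magazine count and recoil, with magazine capacity read from its weapon data asset.
; Firing traces from the camera center, spawns a bullet from the muzzle aimed at that point and ejects a randomly pitched shell, or plays an empty sound.
; A timeline kicks controller pitch with random yaw, then reverses to recover pitch.
; The reload event only plays an animation, without refilling ammo.
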(event Custom|后坐力
  (bind _returnvalue (Game|Player|GetPlayerPawn 0))
  (bind _后坐力yaw (Variables|Default|Get后坐力Yaw))
  ;[1 1 1] 开火
  ;;[1 1 1] 后坐力
  (bind (_direction _新建轨道_0) (Timeline|后坐力释放 PlayFromStart)
    (:Update
      (switch Utilities|FlowControl|Switch|SwitchonETimelineDirection _direction
        (:Forward
          (Pawn|Input|AddControllerPitchInput _returnvalue (Math|Float|Lerp 0.0 (Variables|Default|Get后坐力Pitch) _新建轨道_0))
          (Pawn|Input|AddControllerYawInput _returnvalue (Math|Random|RandomFloatinRange (* _后坐力yaw -1.0) _后坐力yaw)))
        (:Backward
          (Pawn|Input|AddControllerPitchInput (Game|Player|GetPlayerPawn 0) (* (Math|Float|Lerp 0.0 (Variables|Default|Get后坐力Pitch) _新建轨道_0) -1.0)))))
    (:Finished
      (CallFunction|回拉))))

(event Custom|回拉
  (bind _returnvalue (Game|Player|GetPlayerPawn 0))
  (bind _后坐力yaw (Variables|Default|Get后坐力Yaw))
  ;[1 1 1] 开火
  ;;[1 1 1] 后坐力
  (bind (_direction _新建轨道_0) (Timeline|后坐力释放 Reverse)
    (:Update
      (switch Utilities|FlowControl|Switch|SwitchonETimelineDirection _direction
        (:Forward
          (Pawn|Input|AddControllerPitchInput _returnvalue (Math|Float|Lerp 0.0 (Variables|Default|Get后坐力Pitch) _新建轨道_0))
          (Pawn|Input|AddControllerYawInput _returnvalue (Math|Random|RandomFloatinRange (* _后坐力yaw -1.0) _后坐力yaw)))
        (:Backward
          (Pawn|Input|AddControllerPitchInput (Game|Player|GetPlayerPawn 0) (* (Math|Float|Lerp 0.0 (Variables|Default|Get后坐力Pitch) _新建轨道_0) -1.0)))))
    (:Finished
      (CallFunction|回拉))))

(event EventBeginPlay
  (Variables|Default|Set弹匣子弹数 (Variables|/Game/数据资产/武器_数据资产.武器_数据资产_C|Get弹匣上限 (Variables|Default|Get武器数据资产))))

(event Event武器上弹
  (Components|Animation|PlayAnimation (Variables|Default|GetSkeletalMesh) (Variables|Default|Get武器上弹动画) false))

(event Event开火
  (bind _returnvalue (Game|GetPlayerCameraManager 0))
  (bind _skeletalmesh (Variables|Default|GetSkeletalMesh))
  (bind _skeletalmesh_2 (Variables|Default|GetSkeletalMesh))
  (bind _returnvalue_2 (Camera|GetCameraLocation _returnvalue))
  (bind _returnvalue_3 (Transformation|GetSocketTransform _skeletalmesh_2 "Fire_FX_Slot" "RTS_World"))
  (bind _returnvalue_4 (Transformation|GetSocketTransform _skeletalmesh "子弹壳产生" "RTS_World"))
  ;[1 1 1] 开火
  (Components|Animation|PlayAnimation (Variables|Default|GetSkeletalMesh) (Variables|Default|Get武器射击动画) false)
  (if (== (Variables|Default|Get弹匣子弹数) 0)
    (Audio|PlaySoundatLocation "/Game/音效/Empty.Empty" (Transformation|GetActorLocation) "0, 0, 0" 1.0 1.0 0.0 0 0 0 0)
    (else
      (CallFunction|后坐力)
      (Audio|PlaySoundatLocation (Variables|Default|Get开火音效) (Transformation|GetActorLocation) "0, 0, 0" 1.0 1.0 0.0 0 0 0 0)
      (Effects|Components|ParticleSystem|SetTemplate (Variables|Default|Get开火特效) (Variables|Default|Get枪口开火特效))
      (bind (_outhit _returnvalue_5) (Collision|LineTraceByChannel _returnvalue_2 (+ _returnvalue_2 (* (Math|Vector|GetForwardVector (Camera|GetCameraRotation _returnvalue)) 20000)) "TraceTypeQuery5" false 0 "None"))
      (Game|SpawnActorfromClass "/Game/武器蓝图/子弹_BP.子弹_BP_C" (Math|Transform|MakeTransform (.location _returnvalue_3) (Math|Rotator|FindLookatRotation (.location _returnvalue_3) (select _returnvalue_5 (.Location (Collision|BreakHitResult _outhit)) (.TraceEnd (Collision|BreakHitResult _outhit)))) "1.000000,1.000000,1.000000") "AlwaysSpawn" "MultiplyWithRoot" 0 0)
      (Math|Integer|DecrementInt (Variables|Default|Get弹匣子弹数)
        (:%20%20
          (Game|SpawnActorfromClass "/Game/武器蓝图/子弹壳_BP.子弹壳_BP_C" (Math|Transform|MakeTransform (.location _returnvalue_4) (Math|Rotator|MakeRotator (.roll (.rotation _returnvalue_4)) (- (.pitch (.rotation _returnvalue_4)) (Math|Random|RandomFloatinRange -2e+01 45.0)) (.yaw (.rotation _returnvalue_4))) (.scale _returnvalue_4)) "AlwaysSpawn" "MultiplyWithRoot" 0 0))))))

(fn ConstructionScript)

(fn 获取装备的武器数据资产
  (return (Variables|Default|Get武器数据资产)))