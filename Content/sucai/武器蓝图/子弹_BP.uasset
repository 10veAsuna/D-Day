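; Bullet actor Blueprint that plays a surface-specific impact effect when it hits something.
; On Hit, a small sphere trace at the hit location reads the physical surface type and selects the matching directional particle effect.
; Default, metal, concrete and wood surfaces also get a short-lived bullet-hole decal aligned to the surface normal.
; After a successful trace, it spawns the effect along that normal and destroys itself.
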(event Custom|添加弹孔贴花
  (params (Location :type Vector) (Rotation :type Rotator))
  (Rendering|Decal|SpawnDecalatLocation (Variables|Default|Get弹孔贴花材质) "7.000000,7.000000,7.000000" Location Rotation 5.0))

(event EventBeginPlay)

(event Collision|EventHit
  (params (MyComp :type Primitive%20Component%20Object%20Reference) (Other :type Actor%20Object%20Reference) (OtherComp :type Primitive%20Component%20Object%20Reference) (bSelfMoved :type Boolean) (HitLocation :type Vector :default "0, 0, 0") (HitNormal :type Vector :default "0, 0, 0") (NormalImpulse :type Vector :default "0, 0, 0") (Hit :type Hit%20Result%20Structure%20%28by%20ref%29))
  (bind (_outhit _returnvalue) (Collision|SphereTraceByChannel HitLocation HitLocation 3.0 "TraceTypeQuery5" false 0 "None"))
  (if _returnvalue
    (switch Utilities|FlowControl|Switch|SwitchonEPhysicalSurface (Collision|GetSurfaceType _outhit)
      (:SurfaceType_Default
        (Variables|Default|Set命中特效 "/Game/Weapon_Impacts/Systems/Metal/Metal_Impact_Directional_01.Metal_Impact_Directional_01")
        (CallFunction|添加弹孔贴花 (.Location (Collision|BreakHitResult _outhit)) (Math|Conversions|RotationFromXVector (.Normal (Collision|BreakHitResult _outhit))) :!label _label))
      (:SurfaceType1
        (Variables|Default|Set命中特效 "/Game/Weapon_Impacts/Systems/Metal/Metal_Impact_Directional_03.Metal_Impact_Directional_03")
        (goto _label))
      (:SurfaceType2
        (Variables|Default|Set命中特效 "/Game/Weapon_Impacts/Systems/Concrete/Concrete_Impact_Directional_01.Concrete_Impact_Directional_01")
        (goto _label))
      (:SurfaceType3
        (Variables|Default|Set命中特效 "/Game/Weapon_Impacts/Systems/Water/Water_Impact_Directional_01.Water_Impact_Directional_01"))
      (:SurfaceType4
        (Variables|Default|Set命中特效 "/Game/Weapon_Impacts/Systems/Dirt/Dirt_Impact_Directional_01.Dirt_Impact_Directional_01"))
      (:SurfaceType5
        (Variables|Default|Set命中特效 "/Game/Weapon_Impacts/Systems/Wood/Impact_Wood_Directional_01.Impact_Wood_Directional_01")
        (goto _label))
      (:SurfaceType6
        (Variables|Default|Set命中特效 "/Game/Weapon_Impacts/Systems/Grass/Grass_Impact_Directional_01.Grass_Impact_Directional_01"))
      (:SurfaceType7
        (Variables|Default|Set命中特效 "/Game/Weapon_Impacts/Systems/Blood/Blood_Impact_Directional_01.Blood_Impact_Directional_01")))
    (Effects|SpawnEmitteratLocation (Variables|Default|Get命中特效) (.Location (Collision|BreakHitResult _outhit)) (Math|Conversions|RotationFromXVector (.Normal (Collision|BreakHitResult _outhit))))
    (Actor|DestroyActor)))

(fn ConstructionScript)