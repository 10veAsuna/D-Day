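; AI soldier character with a random paratrooper mesh and a camera-facing US or German team label.
; It patrols random reachable points, re-triggered through a delay on Tick, and approaches sensed pawns of the opposing team through an AI interface.
; On arrival it turns and fires a damaging line trace, closing in if the hit lacks the "person" tag.
; Depleted health triggers ragdoll and timed removal.
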(event OnSeePawn(PawnSensing)
  (params (Pawn :type Pawn%20Object%20Reference))
  (if (Utilities|DoesObjectImplementInterface Pawn "/Game/API/API_AI.API_AI_C")
    (bind _team (Class|APIAI|GetAITeam(Message) Pawn))
    (if (Utilities|Enum|NotEqual(Enum) _team (Variables|Default|GetAITeam))
      (bind _output_get (Variables|Default|SetPawn Pawn))
      (CallFunction|AIMoveto _output_get))))

(event Custom|CustomEvent_2
  (params (Pawn :type Pawn%20Object%20Reference))
  (Utilities|IsValid Pawn
    (:Is%20Valid
      (AI|AIMoveTo self "0, 0, 0" Pawn (Variables|Default|GetAcceptance%20Radius_0) false
        (:OnSuccess
          (CallFunction|FacetoPlayer)
          (CallFunction|Fire))))))

(event Custom|CustomEvent
  ;[0.15 0.15 0.15 0.5] 巡逻
  (AI|AIMoveTo self (.RandomLocation (AI|Navigation|GetRandomReachablePointinRadius (Transformation|GetActorLocation) 1e+03 0 0)) 0 5.0 false
    (:OnSuccess
      (Utilities|FlowControl|Delay 1.0))
    (:OnFail
      _))
  (CallFunction|GoonPatrol))

(event Custom|CustomEvent_1
  (bind _mesh (Variables|Character|GetMesh))
  ;[0.15 0.15 0.15 0.5] 随机换装
  (Utilities|FlowControl|MultiGate true false (Math|Random|RandomIntegerinRange 0 3)
    (:Out%200
      (Components|SkeletalMesh|SetSkeletalMeshAsset _mesh "/Game/AlliedMilitaryFigureModel/Meshes/SK_WWII_US_Paratrooper_no_helmet.SK_WWII_US_Paratrooper_no_helmet"))
    (:Out%201
      (Components|SkeletalMesh|SetSkeletalMeshAsset _mesh "/Game/AlliedMilitaryFigureModel/Meshes/SK_WWII_US_Paratrooper_no_helmet_w_equipment.SK_WWII_US_Paratrooper_no_helmet_w_equipment"))
    (:Out%202
      (Components|SkeletalMesh|SetSkeletalMeshAsset _mesh "/Game/AlliedMilitaryFigureModel/Meshes/SK_WWII_US_Paratrooper_simple.SK_WWII_US_Paratrooper_simple"))
    (:Out%203
      (Components|SkeletalMesh|SetSkeletalMeshAsset _mesh "/Game/AlliedMilitaryFigureModel/Meshes/SK_WWII_US_Paratrooper_simpleB.SK_WWII_US_Paratrooper_simpleB"))))

(event Custom|CustomEvent_3
  ;[0.15 0.15 0.15 0.5] 开火
  ;;[0.15 0.15 0.15 0.5] 面向玩家
  (Utilities|IsValid self
    (:Is%20Valid
      (Transformation|SetActorRelativeRotation (Math|Rotator|MakeRotator 0.0 0.0 (.yaw (Math|Rotator|FindLookatRotation (Transformation|GetActorLocation) (Transformation|GetActorLocation (Variables|Default|GetPawn)))))))))

(event Custom|CustomEvent_4
  (bind _arrow1 (Variables|Default|GetArrow1))
  (bind _returnvalue (Transformation|GetWorldLocation _arrow1))
  ;[0.15 0.15 0.15 0.5] 开火
  (Utilities|FlowControl|Delay 0.3)
  (Components|Activation|Activate (Variables|Default|GetNiagara) false)
  (Audio|PlaySoundatLocation "/Game/Anim/Audio/Guns/A_Bren-3.A_Bren-3" (Transformation|GetActorLocation) "0, 0, 0" 1.0 1.0 0.0 0 0 0 0)
  (bind _outhit (Collision|LineTraceByChannel _returnvalue (+ (* (Math|Vector|GetForwardVector (Transformation|GetWorldRotation _arrow1)) 5e+03) _returnvalue) "TraceTypeQuery5" false 0 "ForDuration"))
  (Development|PrintString (Utilities|GetDisplayName (.HitActor (Collision|BreakHitResult _outhit))))
  (bind _returnvalue_2 (Game|Damage|ApplyDamage (.HitActor (Collision|BreakHitResult _outhit)) 5e+01 0 self))
  (Development|PrintString (Utilities|String|ToString(Float) _returnvalue_2))
  (if (not (Actor|ActorHasTag (.HitActor (Collision|BreakHitResult _outhit)) "person"))
    (Variables|Default|SetAcceptance%20Radius_0 (- (Variables|Default|GetAcceptance%20Radius_0) 5e+01))
    (CallFunction|CustomEvent2 (Variables|Default|GetPawn))))

(event Custom|CustomEvent_7
  (bind _returnvalue (Utilities|Name|MakeLiteralName "pelvis"))
  (bind _mesh (Variables|Character|GetMesh))
  (Pawn|Components|CharacterMovement|SetMovementMode (Variables|Character|GetCharacterMovement) "MOVE_None" 0)
  (Collision|SetCollisionProfileName _mesh "ragdoll" true :!class /Script/Engine.PrimitiveComponent)
  (Class|SkeletalMeshComponent|SetAllBodiesBelowSimulatePhysics _mesh _returnvalue true true)
  (Class|SkeletalMeshComponent|SetAllBodiesBelowPhysicsBlendWeight (Variables|Character|GetMesh) _returnvalue 1.0 false true))

(event Custom|CustomEvent_6
  (if (<= (Variables|Default|GetHealth) 0.0)
    (Variables|Default|Setdie? true)
    (CallFunction|EnableRagdoll)
    (Pawn|Components|CharacterMovement|DisableMovement (Variables|Character|GetCharacterMovement))
    (Utilities|FlowControl|Delay 5.0)
    (Utilities|FlowControl|DoOnce false
      (:Completed
        (Actor|SetLifeSpan 5.0)))))

(event Custom|CustomEvent_5
  (bind _aswbp_ainame (Utilities|Casting|CastToWBP_AIName (UserInterface|GetWidget (Variables|Default|GetTeam))))
  (switch Utilities|FlowControl|Switch|SwitchonENUM_Team (Variables|Default|GetAITeam)
    (:NewEnumerator0
      (Rendering|Components|TextRender|SetText (Variables|/Game/AI/AIUI/WBP_AIName.WBP_AIName_C|GetTeam _aswbp_ainame) "US"))
    (:NewEnumerator1
      (Rendering|Components|TextRender|SetText (Variables|/Game/AI/AIUI/WBP_AIName.WBP_AIName_C|GetTeam _aswbp_ainame) "German"))))

(event EventTick
  (params (DeltaSeconds :type Float%20%28single-precision%29))
  ;[0.15 0.15 0.15 0.5] UI面向玩家
  (Transformation|SetWorldRotation (Variables|Default|GetTeam) (Math|Rotator|FindLookatRotation (Transformation|GetActorLocation) (Transformation|GetActorLocation (Game|GetPlayerCameraManager 0))) false false)
  (Utilities|FlowControl|Delay 5.0)
  (CallFunction|GoonPatrol))

(event EventSetAITeam
  (params (Team :type ENUM_Team%20Enum :default "NewEnumerator0"))
  (Variables|Default|SetAITeam Team))

(event Game|Damage|EventAnyDamage
  (params (Damage :type Float%20%28single-precision%29) (DamageType :type Damage%20Type%20Object%20Reference) (InstigatedBy :type Controller%20Object%20Reference) (DamageCauser :type Actor%20Object%20Reference))
  (Variables|Default|SetHealth (- (Variables|Default|GetHealth) Damage))
  (CallFunction|CustomEvent6))

(event EventBeginPlay
  (if (not (Variables|Default|Getdie?))
    (CallFunction|RandomMesh)
    (CallFunction|GoonPatrol)
    (CallFunction|SetTeamText)))

(fn ConstructionScript
  (|CallParentFunction))